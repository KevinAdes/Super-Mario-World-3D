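; PipeBox is a level trigger for Mario pipes that sends the player to another level.
; When BP_Mario begins overlapping its box and the pipe is vertical, not upward and Mario is crouched, it disables his capsule collision.
; After a short delay it opens the configured level by name.
; The crouch check happens only at overlap start, and other pipe orientations have no logic here.
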(event `self.Box.OnComponentBeginOverlap`
  (params (OverlappedComponent :type "PrimitiveComponent Object Reference") (OtherActor :type "Actor Object Reference") (OtherComp :type "PrimitiveComponent Object Reference") (OtherBodyIndex :type Integer) (bFromSweep :type Boolean) (SweepResult :type "HitResult Structure (by ref)"))
  (bind _asmario (cast `/Game/BluePrints/BP_Mario` OtherActor))
  (set `self.As Mario` _asmario)
  (if (`self.Vertical`)
    (if (`self.Up`)
      _
      (elif (`/Game/BluePrints/BP_Mario.Crouched` _asmario)
        (`PrimitiveComponent.SetCollisionEnabled` (`Character.CapsuleComponent` (`self.As Mario`)) "NoCollision")
        (`KismetSystemLibrary.Delay` 3.0)
        (`GameplayStatics.OpenLevel` (`self.LevelToLoad`))))))

(fn `UserConstructionScript`)