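; BP_OneWayPlatform is a platform that BP_Mario can pass through from below and stand on from above.
; Box overlap with Mario stores a reference and enables actor tick, and ending the overlap disables it.
; While ticking, it compares the world height of Mario's Shoebox to that of Box, setting the mesh's GameTraceChannel1 response to Ignore when lower and Block otherwise.
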(event `self.ReceiveTick`
  (params (DeltaSeconds :type "Float (single-precision)"))
  (bind (_returnvalue_x _returnvalue_y _returnvalue_z) (`KismetMathLibrary.BreakVector` (`SceneComponent.K2_GetComponentLocation` (`self.Box`))))
  (bind (_returnvalue_x_2 _returnvalue_y_2 _returnvalue_z_2) (`KismetMathLibrary.BreakVector` (`SceneComponent.K2_GetComponentLocation` (`/Game/BluePrints/BP_Mario.Shoebox` (`self.MarioRef`)))))
  (`PrimitiveComponent.SetCollisionResponseToChannel` (`self.StaticMeshComponent0`) "ECC_GameTraceChannel1" (select `bool` (< _returnvalue_z_2 _returnvalue_z) :`false` "ECR_Block" :`true` "ECR_Ignore" :!type "ECollisionResponse Enum")))

(event `self.Box.OnComponentBeginOverlap`
  (params (OverlappedComponent :type "PrimitiveComponent Object Reference") (OtherActor :type "Actor Object Reference") (OtherComp :type "PrimitiveComponent Object Reference") (OtherBodyIndex :type Integer) (bFromSweep :type Boolean) (SweepResult :type "HitResult Structure (by ref)"))
  (bind _asbp_mario (cast `/Game/BluePrints/BP_Mario` OtherActor))
  (set `self.MarioRef` _asbp_mario)
  (`self.SetActorTickEnabled` true))

(event `self.Box.OnComponentEndOverlap`
  (params (OverlappedComponent :type "PrimitiveComponent Object Reference") (OtherActor :type "Actor Object Reference") (OtherComp :type "PrimitiveComponent Object Reference") (OtherBodyIndex :type Integer))
  (cast `/Game/BluePrints/BP_Mario` OtherActor)
  (`self.SetActorTickEnabled` false))

(fn `UserConstructionScript`)