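; Path actor that moves a ReferencePoint component along its spline at a set speed, looping endlessly.
; Each Tick advances or reduces a distance by Speed, backwards when FlipDir is set, and places ReferencePoint at that spline transform in local space.
; Reverse travel turns the yaw by 180 degrees, and the distance wraps to the opposite end when it passes either end of the spline.
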(event `self.ReceiveTick`
  (params (DeltaSeconds :type "Float (single-precision)"))
  (bind _reference_point (`self.Reference point`))
  (bind _distance (`self.Distance`))
  (bind _distance_2 (`self.Distance`))
  (bind (_returnvalue_location _returnvalue_rotation) (`KismetMathLibrary.BreakTransform` (`SplineComponent.GetTransformAtDistanceAlongSpline` (`self.Spline`) _distance "Local" false)))
  (bind _returnvalue (`SplineComponent.GetSplineLength` (`self.Spline`)))
  (bind _returnvalue_2 (* DeltaSeconds (`self.Speed`)))
  (if (`self.FlipDir`)
    (set `self.Distance` (- _distance _returnvalue_2))
    (`SceneComponent.K2_SetRelativeTransform` _reference_point (`KismetMathLibrary.MakeTransform` _returnvalue_location (`KismetMathLibrary.MakeRotator` (.roll _returnvalue_rotation) (.pitch _returnvalue_rotation) (- (.yaw _returnvalue_rotation) 180.0))) false false)
    (else
      (set `self.Distance` (+ _returnvalue_2 _distance))
      (`SceneComponent.K2_SetRelativeTransform` _reference_point (`KismetMathLibrary.MakeTransform` _returnvalue_location _returnvalue_rotation) false false)))
  (if (> _distance_2 _returnvalue)
    (set `self.Distance` 0.0)
    (elif (< _distance_2 0.0)
      (set `self.Distance` _returnvalue))))

(fn `UserConstructionScript`)