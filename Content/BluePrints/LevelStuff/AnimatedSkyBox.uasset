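; AnimatedSkyBox is a level actor that plays a flipbook-style animated sky by swapping materials on its skybox mesh.
; The construction script applies the first material in the Materials array.
; At BeginPlay a non-looping timer, timed from FramesPerSecond, calls SetNextFrame, which sets the current material, advances the index with modulo wrap-around and re-arms the timer to loop endlessly.
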(event `self.ReceiveBeginPlay`
  (`KismetSystemLibrary.K2_SetTimerDelegate` (delegate `SetNextFrame`) (/ 1.0 (`self.Frames Per Second`)) :!label _label))

(event `SetNextFrame`
  (bind _materials (`self.Materials`))
  (bind _material_index (`self.Material Index`))
  (`PrimitiveComponent.SetMaterial` (`self.SkyboxMesh`) 0 (`|GetArrayItem` _materials _material_index))
  (set `self.Material Index` (mod (+ _material_index 1) (`KismetArrayLibrary.Array_Length` _materials)))
  (goto _label))

(fn `UserConstructionScript`
  (`PrimitiveComponent.SetMaterial` (`self.SkyboxMesh`) 0 (`|GetArrayItem` (`self.Materials`))))