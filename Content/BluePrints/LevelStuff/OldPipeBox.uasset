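; An overlap-triggered pipe entrance that warps BP_Mario to another spawn point while streaming a level in or out.
; Vertical, non-Up pipes require crouching and disable the capsule's collision; horizontal pipes require movement roughly matching the box's forward vector, compared only on Y.
; After a delay, a HUD fade and mosaic effect cover the warp.
; IsSubLevel selects whether the named level unloads or loads, without blocking, as Mario is pseudo-spawned at NextSpawnPoint.
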(event `Warp`
  (bind _as_mario (`self.As Mario`))
  (`KismetSystemLibrary.Delay` 1.0)
  (`|ExecutionSequence`
    (:`then_0`
      (if (`self.isSubLevel`)
        (`/Game/BluePrints/BP_Mario.PsuedoSpawn` (`self.As Mario`) (`self.NextSpawnPoint`))
        (`GameplayStatics.UnloadStreamLevel` (`self.LevelToLoad`))
        (else
          (`GameplayStatics.LoadStreamLevel` (`self.LevelToLoad`) true)
          (`/Game/BluePrints/BP_Mario.PsuedoSpawn` (`self.As Mario`) (`self.NextSpawnPoint`)))))
    (:`then_1`
      (`/Game/BluePrints/Widgets/HUD/WBP_MarioHud.FadeIn` (`/Game/BluePrints/BP_Mario.Mario Hud` _as_mario))
      (`/Game/BluePrints/BP_Mario.Mosaic Out` _as_mario))))

(event `self.Box.OnComponentBeginOverlap`
  (params (OverlappedComponent :type "PrimitiveComponent Object Reference") (OtherActor :type "Actor Object Reference") (OtherComp :type "PrimitiveComponent Object Reference") (OtherBodyIndex :type Integer) (bFromSweep :type Boolean) (SweepResult :type "HitResult Structure (by ref)"))
  (bind _as_mario (`self.As Mario`))
  (bind (_in_vector_x _in_vector_y) (`KismetMathLibrary.BreakVector` (`self.In Vector`)))
  (bind _as_mario_2 (`self.As Mario`))
  (bind _asbp_mario (cast `/Game/BluePrints/BP_Mario` OtherActor))
  (set `self.As Mario` _asbp_mario)
  (if (`self.Vertical`)
    (if (`self.Up`)
      _
      (elif (`/Game/BluePrints/BP_Mario.Crouched` _asbp_mario)
        (`PrimitiveComponent.SetCollisionEnabled` (`Character.CapsuleComponent` (`self.As Mario`)) "NoCollision")
        (`KismetSystemLibrary.Delay` 2.0)
        (`/Game/BluePrints/Widgets/HUD/WBP_MarioHud.FadeOut` (`/Game/BluePrints/BP_Mario.Mario Hud` _as_mario_2))
        (`/Game/BluePrints/BP_Mario.Mosaic In` _as_mario_2)
        (`self.Warp`)))
    (elif (< (`KismetMathLibrary.Abs` (- _in_vector_y (.y (`KismetMathLibrary.Normal` (`CharacterMovementComponent.GetLastUpdateVelocity` (`Character.CharacterMovement` (`self.As Mario`))))))) 0.2)
      (`KismetSystemLibrary.Delay` 2.0)
      (`/Game/BluePrints/Widgets/HUD/WBP_MarioHud.FadeOut` (`/Game/BluePrints/BP_Mario.Mario Hud` _as_mario))
      (`/Game/BluePrints/BP_Mario.Mosaic In` _as_mario)
      (`self.Warp`))))

(fn `UserConstructionScript`
  (set `self.In Vector` (`SceneComponent.GetForwardVector` (`self.Box`))))