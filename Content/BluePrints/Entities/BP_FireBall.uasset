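; BP_FireBall is a Mario-style bouncing fireball projectile that burns flammable actors.
; Tick applies capped gravity, line-traces downward to bounce and forward to detect walls, then moves the actor by manual location offsets.
; Wall hits and overlaps with BPI_Flammable actors spawn a Niagara poof and destroy it, with overlaps also passing scaled horizontal motion to Burn.
; Helper functions spin the mesh and despawn the fireball far from BP_Mario.
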(event `self.ReceiveBeginPlay`
  (set `self.Horizontal Move` (* (`SceneComponent.GetForwardVector` (`self.DefaultSceneRoot`)) 36))
  (`KismetSystemLibrary.K2_SetTimerDelegate` (`|CreateDelegate` :!event `ApplyRotation`) 0.1 true)
  (`KismetSystemLibrary.K2_SetTimerDelegate` (`|CreateDelegate` :!event `CheckMarioDistance`) 0.6 true))

(event `self.ReceiveTick`
  (params (DeltaSeconds :type "Float (single-precision)"))
  (bind (_returnvalue_location _returnvalue_rotation) (`KismetMathLibrary.BreakTransform` (`self.GetTransform`)))
  (bind _returnvalue (`self.K2_GetActorLocation`))
  (bind _returnvalue_2 (`self.K2_GetActorLocation`))
  (`|ExecutionSequence`
    (:`then_0`
      (`self.ApplyGravity`))
    (:`then_1`
      (bind (_outhit _returnvalue_3) (`KismetSystemLibrary.LineTraceSingleForObjects` _returnvalue (+ _returnvalue (`KismetMathLibrary.MakeVector` 0.0 0.0 (`self.VerticalMove`))) (`|MakeArray` "ObjectTypeQuery1" "ObjectTypeQuery2" :!type "EObjectTypeQuery Enum")))
      (if _returnvalue_3
        (set `self.VerticalMove` 40.0)))
    (:`then_2`
      (bind (_outhit_2 _returnvalue_4) (`KismetSystemLibrary.LineTraceSingleForObjects` _returnvalue_2 (+ _returnvalue_2 (`self.Horizontal Move`)) (`|MakeArray` "ObjectTypeQuery1" "ObjectTypeQuery2" :!type "EObjectTypeQuery Enum")))
      (if _returnvalue_4
        (`self.Poof` _returnvalue_location _returnvalue_rotation)))
    (:`then_3`
      (`self.K2_SetActorLocation` (+ (`self.K2_GetActorLocation`) (+ (`self.Horizontal Move`) (`KismetMathLibrary.MakeVector` 0.0 0.0 (`self.VerticalMove`))))))))

(event `self.Sphere.OnComponentBeginOverlap`
  (params (OverlappedComponent :type "PrimitiveComponent Object Reference") (OtherActor :type "Actor Object Reference") (OtherComp :type "PrimitiveComponent Object Reference") (OtherBodyIndex :type Integer) (bFromSweep :type Boolean) (SweepResult :type "HitResult Structure (by ref)"))
  (bind (_returnvalue_location _returnvalue_rotation) (`KismetMathLibrary.BreakTransform` (`self.GetTransform` OtherActor)))
  (bind _asbpi_flammable (cast `/Game/BluePrints/Interfaces/BPI_Flammable` OtherActor))
  (`self.Poof` _returnvalue_location _returnvalue_rotation)
  (`/Game/BluePrints/Interfaces/BPI_Flammable.Burn` _asbpi_flammable (* (`self.Horizontal Move`) 0.2)))

(event `self.Niagara.OnSystemFinished`
  (params (PSystem :type "NiagaraComponent Object Reference")))

(fn `ApplyGravity`
  (bind _returnvalue (- (`self.VerticalMove`) 3.85))
  (set `self.VerticalMove` (`KismetMathLibrary.SelectFloat` -24.0 _returnvalue (<= _returnvalue -24.0))))

(fn `ApplyRotation`
  (bind _staticmesh (`self.StaticMesh`)
    (:`then`
      (`SceneComponent.K2_AddLocalRotation` _staticmesh (struct :`Pitch` -90.0) false false))
    (:`else`)))

(fn `CheckMarioDistance`
  (bind (_returnvalue_location _returnvalue_rotation) (`KismetMathLibrary.BreakTransform` (`self.GetTransform`)))
  (bind _returnvalue (`GameplayStatics.GetActorOfClass` "/Game/BluePrints/BP_Mario.BP_Mario_C"))
  (if (>= (`KismetMathLibrary.Vector_Distance2D` (`self.K2_GetActorLocation` _returnvalue) (`self.K2_GetActorLocation` self)) 2000.0)
    (`self.Poof` _returnvalue_location _returnvalue_rotation)))

(fn `Poof`
  (params (Location :type "Vector Structure") (Rotation :type "Rotator Structure"))
  (`NiagaraFunctionLibrary.SpawnSystemAtLocation` "/Game/Particles/Systems/NS_Poof.NS_Poof" Location Rotation (1.0 1.0 1.0) false)
  (`self.K2_DestroyActor`))

(fn `UserConstructionScript`)