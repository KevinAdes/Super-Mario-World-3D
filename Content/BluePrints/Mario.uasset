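; Player character Blueprint for Mario, with camera-relative walking, timed run-to-sprint, skidding, crouch, look-up, jump and spin jump.
; Animation swaps whole skeletal meshes on Delay loops, with movement state choosing the Meshes indices.
; Jumps set launch velocity by speed state and retune GravityScale on press, release and apex for variable arcs.
; A spring-arm camera supports manual yaw, timeline-driven zoom and height, and smooth reset toward Mario's facing.
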(event `FixSkidRotValues`
  (bind _mariodirection (`self.MarioDirection`))
  (bind _yaw (.yaw (`SceneComponent.K2_GetComponentRotation` (`self.Mesh`))))
  (if (< _mariodirection 0.0)
    (set `self.CurrentDirectionRotCheck` (+ _mariodirection 360.0))
    (else
      (set `self.CurrentDirectionRotCheck` _mariodirection)))
  (if (< _yaw 0.0)
    (set `self.FutureDirectionRotCheck` (+ _yaw 360.0))
    (else
      (set `self.FutureDirectionRotCheck` _yaw))))

(event `InputAxis|MoveForward`
  (params (AxisValue :type "Float (single-precision)"))
  (bind _returnvalue (!= AxisValue 0.0))
  (bind _step_duration (`self.Step Duration`))
  (bind _mesh (`self.Mesh`))
  (bind _mesh_2 (`self.Mesh`))
  (bind _step_duration_2 (`self.Step Duration`))
  (bind _returnvalue_2 (or (`self.Crouched`) (`self.LookingUp`) (`self.Jumping`) (`self.Skidding`)))
  (bind _returnvalue_3 (`KismetMathLibrary.Abs` (- (`self.CurrentDirectionRotCheck`) (`self.FutureDirectionRotCheck`))))
  (bind _returnvalue_4 (and (`self.Walking`) (not (`self.Skidding`))))
  (bind _returnvalue_5 (and (`self.Walking`) (not (`self.Skidding`))))
  (bind _returnvalue_6 (`KismetMathLibrary.MakeRotator` 0.0 0.0 (.yaw (`SceneComponent.K2_GetComponentRotation` (`self.Camera`)))))
  (bind _returnvalue_7 (`KismetMathLibrary.GetForwardVector` _returnvalue_6))
  (bind _returnvalue_8 (`KismetMathLibrary.GetRightVector` _returnvalue_6))
  (bind _returnvalue_9 (* AxisValue _returnvalue_7))
  (if (and (`self.NewMacro_0`) _returnvalue)
    (if (not (`self.SpinJumping`)) :!label _label
      (bind _returnvalue_10 (* (stale `InputAxis|Move Right` AxisValue) _returnvalue_8))
      (`SceneComponent.K2_SetWorldRotation` (`self.Mesh`) (`KismetMathLibrary.Conv_VectorToRotator` (+ _returnvalue_9 _returnvalue_10)) false false)
      (`self.FixSkidRotValues`)
      (if (and (and (>= _returnvalue_3 45.0) (< _returnvalue_3 350.0)) (not (`self.Jumping`)))
        (`SkinnedMeshComponent.SetSkinnedAssetAndUpdate` (`self.Mesh`) "/Game/Models/Mario/Small/Skid.Skid" true)
        (set `self.Skidding` true)
        (`self.SkidReset`)
        (set `CharacterMovementComponent.bCanWalkOffLedges` false (`self.CharacterMovement`))
        (`self.AddMovementInput` (`self.MoveVector1`) 0.5)
        (`self.AddMovementInput` (`self.MoveVector2`) 0.5)
        (`KismetSystemLibrary.Delay` 0.5)
        (set `self.Skidding` false)
        (set `CharacterMovementComponent.bCanWalkOffLedges` true (`self.CharacterMovement`)))
      (set `self.MarioDirection` (.yaw (`SceneComponent.K2_GetComponentRotation` (`self.Mesh`))))
      (set `self.MoveVector1` _returnvalue_9)
      (set `self.MoveVector2` _returnvalue_10))
    (`self.AddMovementInput` _returnvalue_7 AxisValue)
    (`self.AddMovementInput` _returnvalue_8 (stale `InputAxis|Move Right` AxisValue))
    (if (not _returnvalue_2)
      (set `self.Walking` true)
      (if (not (`self.Walking(Animation)`))
        (set `self.Walking(Animation)` true)
        (`SkinnedMeshComponent.SetSkinnedAssetAndUpdate` _mesh (`|GetArrayItem` (`self.Meshes`) (`self.MovementStep`)) false :!label _label_2)
        (`KismetSystemLibrary.Delay` _step_duration_2)
        (if _returnvalue_5
          (`SkinnedMeshComponent.SetSkinnedAssetAndUpdate` _mesh (`|GetArrayItem` (`self.Meshes`) (`self.MovementStill`)) false)
          (`KismetSystemLibrary.Delay` _step_duration_2)
          (if _returnvalue_5
            (`SkinnedMeshComponent.SetSkinnedAssetAndUpdate` _mesh_2 (`|GetArrayItem` (`self.Meshes`) (`self.MovementStep2`)) false)
            (`KismetSystemLibrary.Delay` _step_duration)
            (if _returnvalue_4
              (`SkinnedMeshComponent.SetSkinnedAssetAndUpdate` _mesh_2 (`|GetArrayItem` (`self.Meshes`) (`self.MovementStill`)) false)
              (`KismetSystemLibrary.Delay` _step_duration)
              (if _returnvalue_4
                (goto _label_2)
                (else
                  _)))))
        (set `self.Walking(Animation)` false)))
    (else
      (if (and (not _returnvalue) (not (!= (stale `InputAxis|Move Right` AxisValue) 0.0)) (not _returnvalue_2)) :!label _label_3
        (set `self.Walking` false)
        (`SkinnedMeshComponent.SetSkinnedAssetAndUpdate` (`self.Mesh`) "/Game/Models/Mario/Small/Idle.Idle" true)))))

(event `InputAxis|Move Right`
  (params (AxisValue :type "Float (single-precision)"))
  (if (and (!= AxisValue 0.0) (`self.NewMacro_0`))
    (goto _label)
    (else
      (goto _label_3))))

(event `InputAxis|Turn`
  (params (AxisValue :type "Float (single-precision)"))
  ;[1 1 1] Camera Controls
  (`SceneComponent.K2_AddWorldRotation` (`self.SpringArm`) (`KismetMathLibrary.MakeRotator` 0.0 0.0 AxisValue) false false))

(event `InputAxis|CameraUp`
  (params (AxisValue :type "Float (single-precision)"))
  ;[1 1 1] Camera Controls
  (bind _output_get (set `self.CameraTime` (+ (* AxisValue 0.1) (`self.CameraTime`))))
  (bind (_direction _springarm_scale _camera_rotation _camera_height) (`Timeline|Camera Zoom` :`NewTime` _output_get :!via `SetNewTime`)
    (:`Update`
      (`SceneComponent.SetRelativeScale3D` (`self.SpringArm`) (`KismetMathLibrary.Conv_DoubleToVector` _springarm_scale))
      (`SceneComponent.K2_SetRelativeLocationAndRotation` (`self.Camera`) (`KismetMathLibrary.MakeVector` -1255.369049 0.0 _camera_height) (`KismetMathLibrary.MakeRotator` 0.0 _camera_rotation) false false))))

(event `InputAction|Reset Cam`
  (params (Key :type "Key Structure"))
  (bind _springarm (`self.SpringArm`))
  (bind (_relativerotation_roll _relativerotation_pitch _relativerotation_yaw) (`KismetMathLibrary.BreakRotator` (`SceneComponent.RelativeRotation` _springarm)))
  ;[1 1 1] Camera Controls
  (:`Pressed`
    (`self.FixRotValues`)
    (set `self.CamRotating` 0)
    (bind _output_get (set `self.SpringArmTempRot` _relativerotation_yaw))
    (bind (_direction _smooth) (`Timeline|SmoothRot` :!via `PlayFromStart`)
      (:`Update`
        (`SceneComponent.K2_SetRelativeRotation` _springarm (`KismetMathLibrary.MakeRotator` 0.0 0.0 (+ _output_get (* _smooth (- (`self.MarioRotCheck`) (`self.SpringArmRotCheck`))))) true false)
        (set `self.CamRotating` 1)))))

(event `InputAction|Crouch`
  (params (Key :type "Key Structure"))
  (bind _jumping (`self.Jumping`))
  (bind _mesh (`self.Mesh`))
  (:`Pressed`
    (set `self.Crouched` true)
    (if (not _jumping)
      (set `self.Walking` false)
      (set `self.MovementJump` 9)
      (set `self.MovementFall` 9)
      (`SkinnedMeshComponent.SetSkinnedAssetAndUpdate` _mesh "/Game/Models/Mario/Small/Crouch.Crouch" true)
      (`SceneComponent.K2_SetRelativeLocation` _mesh (0.0 0.0 -34.0) false false)))
  (:`Released`
    (set `self.Crouched` false)
    (if (not _jumping)
      (set `self.MovementJump` 2)
      (set `self.MovementFall` 3)
      (`SceneComponent.K2_SetRelativeLocation` _mesh (0.0 0.0 0.0) false false)
      (if (`self.LookingUp`)
        (set `self.LookingUp` true :!label _label_4)
        (if (not (or (`self.Crouched`) (`self.Jumping`)))
          (set `self.Walking` false)
          (set `self.MovementJump` 2)
          (set `self.MovementFall` 3)
          (`SkinnedMeshComponent.SetSkinnedAssetAndUpdate` (`self.Mesh`) "/Game/Models/Mario/Small/LookUp.LookUp" true))
        (else
          (`SkinnedMeshComponent.SetSkinnedAssetAndUpdate` _mesh "/Game/Models/Mario/Small/Idle.Idle" true))))))

(event `InputAction|LookUp`
  (params (Key :type "Key Structure"))
  (:`Pressed`
    (goto _label_4))
  (:`Released`
    (set `self.LookingUp` false)))

(event `InputAction|Debug`
  (params (Key :type "Key Structure"))
  (:`Pressed`
    (`KismetSystemLibrary.PrintString` (`KismetStringLibrary.Conv_DoubleToString` (`KismetMathLibrary.DegAcos` (`KismetMathLibrary.Dot_VectorVector` (`.ImpactNormal` (`GameplayStatics.BreakHitResult` (`.HitResult` (break `FindFloorResult` (`CharacterMovementComponent.CurrentFloor` (`self.CharacterMovement`)))))) (0.0 0.0 1.0)))))))

(event `FixRotValues`
  (bind _yaw (.yaw (`SceneComponent.K2_GetComponentRotation` (`self.SpringArm`))))
  (bind _yaw_2 (.yaw (`SceneComponent.K2_GetComponentRotation` (`self.Mesh`))))
  ;[1 1 1] Camera Controls
  (if (< _yaw 0.0)
    (set `self.SpringArmRotCheck` (+ _yaw 360.0))
    (else
      (set `self.SpringArmRotCheck` _yaw)))
  (if (< _yaw_2 0.0)
    (set `self.MarioRotCheck` (+ _yaw_2 360.0))
    (else
      (set `self.MarioRotCheck` _yaw_2))))

(event `InputAction|Run2`
  (params (Key :type "Key Structure"))
  (bind _runbuttoncount (`self.RunButtonCount`))
  (bind _charactermovement (`self.CharacterMovement`))
  (:`Pressed`
    (bind _result (`/Engine/EditorBlueprintResources/StandardMacros.IncrementInt` _runbuttoncount :!label _label_5)
      (:`  `
        (if (not (> _result 1))
          (set `self.runheld` true)
          (set `self.Step Duration` 0.1 :!label _label_6)
          (set `CharacterMovementComponent.MaxWalkSpeed` 1560.0 _charactermovement)
          (set `self.MovementStep` 0)
          (set `self.MovementStep2` 11)
          (set `self.MovementStill` 1)
          (set `self.MovementJump` 2)
          (set `self.MovementFall` 3)
          (`KismetSystemLibrary.Delay` 2.0)
          (if (`self.runheld`)
            (set `CharacterMovementComponent.MaxWalkSpeed` 2000.0 _charactermovement)
            (set `self.Step Duration` 0.05)
            (set `self.Sprinting` true)
            (set `self.MovementStep` 4)
            (set `self.MovementStep2` 12)
            (set `self.MovementStill` 5)
            (set `self.MovementJump` 6)
            (set `self.MovementFall` 6))))))
  (:`Released`
    (bind _result_2 (`/Engine/EditorBlueprintResources/StandardMacros.DecrementInt` _runbuttoncount :!label _label_7)
      (:`  `
        (if (== _result_2 0)
          (set `self.runheld` false)
          (set `self.Step Duration` 0.2 :!label _label_8)
          (set `CharacterMovementComponent.MaxWalkSpeed` 844.0 _charactermovement)
          (set `self.Sprinting` false)
          (set `self.MovementStep` 0)
          (set `self.MovementStep2` 11)
          (set `self.MovementStill` 1)
          (set `self.MovementJump` 2)
          (set `self.MovementFall` 3))))))

(event `InputAction|Run`
  (params (Key :type "Key Structure"))
  (:`Pressed`
    (goto _label_5))
  (:`Released`
    (goto _label_7)))

(event `SkidReset`
  (if (== (`self.RunButtonCount`) 0)
    (goto _label_8)
    (else
      (goto _label_6))))

(event `InputAction|Jump`
  (params (Key :type "Key Structure"))
  (bind _charactermovement (`self.CharacterMovement`))
  (bind _charactermovement_2 (`self.CharacterMovement`))
  (bind _mesh (`self.Mesh`))
  (bind _charactermovement_3 (`self.CharacterMovement`))
  (bind _charactermovement_4 (`self.CharacterMovement`))
  (:`Pressed`
    (`SceneComponent.K2_SetRelativeLocation` (`self.Mesh`) (0.0 0.0 0.0) false false)
    (set `CharacterMovementComponent.bNotifyApex` true _charactermovement_4)
    (add `self.OnReachedJumpApex` (delegate `OnReachedJumpApex_Event_0`))
    (if (`self.Jumping`)
      (if (`self.Sprinting`)
        (set `CharacterMovementComponent.GravityScale` 6.8 _charactermovement_4)
        (elif (`self.Walking`)
          (set `CharacterMovementComponent.GravityScale` 6.7 _charactermovement_4)
          (else
            (set `CharacterMovementComponent.GravityScale` 6.5 _charactermovement_4))))
      (else
        (set `self.Jumping` true)
        (set `self.Walking` false)
        (`SceneComponent.SetRelativeScale3D` _mesh (1.0 1.0 1.0))
        (`SkinnedMeshComponent.SetSkinnedAssetAndUpdate` _mesh (`|GetArrayItem` (`self.Meshes`) (`self.MovementJump`)) false)
        (if (`self.Apex Reached`)
          (if (`self.Sprinting`) :!label _label_9
            (set `CharacterMovementComponent.GravityScale` 7.05 _charactermovement_3)
            (elif (`self.Walking`)
              (set `CharacterMovementComponent.GravityScale` 6.82 _charactermovement_3)
              (else
                (set `CharacterMovementComponent.GravityScale` 6.6 _charactermovement_3))))
          (`SkinnedMeshComponent.SetSkinnedAssetAndUpdate` (`self.Mesh`) (`|GetArrayItem` (`self.Meshes`) (`self.MovementFall`)) true)
          (else
            (if (`self.Sprinting`)
              (set `CharacterMovementComponent.GravityScale` 6.8 _charactermovement_4)
              (set `CharacterMovementComponent.JumpZVelocity` 3470.0 _charactermovement_4)
              (elif (`self.Walking`)
                (set `CharacterMovementComponent.GravityScale` 6.7 _charactermovement_4)
                (set `CharacterMovementComponent.JumpZVelocity` 3220.0 _charactermovement_4)
                (else
                  (set `CharacterMovementComponent.GravityScale` 6.5 _charactermovement_4)
                  (set `CharacterMovementComponent.JumpZVelocity` 2960.0 _charactermovement_4))))
            (`self.Jump`))))))
  (:`Released`
    (if (`self.Apex Reached`)
      (if (`self.Sprinting`)
        (set `CharacterMovementComponent.GravityScale` 8.35 _charactermovement)
        (elif (`self.Walking`)
          (set `CharacterMovementComponent.GravityScale` 13.61 _charactermovement)
          (else
            (set `CharacterMovementComponent.GravityScale` 12.43 _charactermovement))))
      (`self.StopJumping`)
      (else
        (if (`self.Sprinting`)
          (set `CharacterMovementComponent.GravityScale` 12.17 _charactermovement_2)
          (elif (`self.Walking`)
            (set `CharacterMovementComponent.GravityScale` 13.06 _charactermovement_2)
            (else
              (set `CharacterMovementComponent.GravityScale` 12.08 _charactermovement_2))))
        (`self.StopJumping`)))))

(event `self.OnLanded`
  (params (Hit :type "HitResult Structure (by ref)"))
  (bind _mesh (`self.Mesh`))
  (bind _mesh_2 (`self.Mesh`))
  (bind _mesh_3 (`self.Mesh`))
  (set `self.Apex Reached` false)
  (set `self.SpinJumping` false)
  (set `self.Jumping` false)
  (if (`self.Crouched`)
    (set `self.Walking` false)
    (set `self.MovementJump` 9)
    (set `self.MovementFall` 9)
    (`SkinnedMeshComponent.SetSkinnedAssetAndUpdate` _mesh "/Game/Models/Mario/Small/Crouch.Crouch" true)
    (`SceneComponent.K2_SetRelativeLocation` _mesh (0.0 0.0 -34.0) false false)
    (elif (`self.LookingUp`)
      (set `self.Walking` false)
      (set `self.MovementJump` 2)
      (set `self.MovementFall` 3)
      (`SkinnedMeshComponent.SetSkinnedAssetAndUpdate` _mesh_2 "/Game/Models/Mario/Small/LookUp.LookUp" true)
      (`SceneComponent.K2_SetRelativeLocation` _mesh_2 (0.0 0.0 0.0) false false)
      (else
        (if (`self.Sprinting`)
          (set `self.MovementJump` 6)
          (set `self.MovementFall` 6)
          (else
            (set `self.MovementJump` 2)
            (set `self.MovementFall` 3)))
        (`SkinnedMeshComponent.SetSkinnedAssetAndUpdate` _mesh_3 "/Game/Models/Mario/Small/Idle.Idle" true)
        (`SceneComponent.K2_SetRelativeLocation` _mesh_3 (0.0 0.0 0.0) false false)))))

(event `OnReachedJumpApex_Event_0`
  (bind _charactermovement (`self.CharacterMovement`))
  (set `self.Apex Reached` true)
  (if (`self.SpinJumping`)
    (if (`self.Sprinting`) :!label _label_10
      (set `CharacterMovementComponent.GravityScale` 5.1 _charactermovement)
      (elif (`self.Walking`)
        (set `CharacterMovementComponent.GravityScale` 5.9 _charactermovement)
        (else
          (set `CharacterMovementComponent.GravityScale` 6.6 _charactermovement))))
    (else
      (goto _label_9))))

(event `InputAction|Spin Jump`
  (params (Key :type "Key Structure"))
  (bind _mesh (`self.Mesh`))
  (bind _charactermovement (`self.CharacterMovement`))
  (bind _charactermovement_2 (`self.CharacterMovement`))
  (:`Pressed`
    (`SceneComponent.K2_SetRelativeLocation` (`self.Mesh`) (0.0 0.0 0.0) false false)
    (if (`self.Jumping`)
      (if (`self.Sprinting`)
        (set `CharacterMovementComponent.GravityScale` 5.55 _charactermovement_2)
        (elif (`self.Walking`)
          (set `CharacterMovementComponent.GravityScale` 6.5 _charactermovement_2)
          (else
            (set `CharacterMovementComponent.GravityScale` 6.5 _charactermovement_2))))
      (else
        (set `self.SpinJumping` true)
        (set `self.Jumping` true)
        (set `self.Walking` false)
        (`SceneComponent.SetRelativeScale3D` _mesh (1.0 1.0 1.0))
        (`SkinnedMeshComponent.SetSkinnedAssetAndUpdate` _mesh "/Game/Models/Mario/Small/Idle.Idle" false)
        (if (`self.Apex Reached`)
          (goto _label_10)
          (else
            (if (`self.Sprinting`)
              (set `CharacterMovementComponent.GravityScale` 5.55 _charactermovement_2)
              (set `CharacterMovementComponent.JumpZVelocity` 2970.0 _charactermovement_2)
              (elif (`self.Walking`)
                (set `CharacterMovementComponent.GravityScale` 6.5 _charactermovement_2)
                (set `CharacterMovementComponent.JumpZVelocity` 2820.0 _charactermovement_2)
                (else
                  (set `CharacterMovementComponent.GravityScale` 6.5 _charactermovement_2)
                  (set `CharacterMovementComponent.JumpZVelocity` 2750.0 _charactermovement_2))))
            (`self.Jump`)
            (if (`self.SpinJumping`) :!label _label_11
              (`SceneComponent.K2_AddLocalRotation` (`self.Mesh`) (struct :`Yaw` 90.0) false false)
              (`KismetSystemLibrary.DelayUntilNextTick`)
              (`KismetSystemLibrary.DelayUntilNextTick`)
              (`KismetSystemLibrary.DelayUntilNextTick`)
              (`KismetSystemLibrary.DelayUntilNextTick`)
              (goto _label_11)))))))
  (:`Released`
    (if (`self.Apex Reached`)
      (if (`self.Sprinting`)
        (set `CharacterMovementComponent.GravityScale` 6.08 _charactermovement_2)
        (elif (`self.Walking`)
          (set `CharacterMovementComponent.GravityScale` 7.48 _charactermovement_2)
          (else
            (set `CharacterMovementComponent.GravityScale` 10.8 _charactermovement_2))))
      (`self.StopJumping`)
      (else
        (if (`self.Sprinting`)
          (set `CharacterMovementComponent.GravityScale` 12.96 _charactermovement)
          (elif (`self.Walking`)
            (set `CharacterMovementComponent.GravityScale` 12.19 _charactermovement)
            (else
              (set `CharacterMovementComponent.GravityScale` 13.6 _charactermovement))))
        (`self.StopJumping`)))))

(fn `UserConstructionScript`)