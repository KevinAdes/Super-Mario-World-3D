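; DragonCoin_BP is a coin item that shimmers in place and disappears when touched.
; From BeginPlay, an endless Delay loop ping-pongs the mesh through four yellow materials to fake an animated shine without Tick.
; Any overlap with the Box component destroys the actor, with no check on the overlapping actor and no score or reward logic.
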(event `self.ReceiveBeginPlay`
  (bind _mesh (`self.Mesh`))
  (`PrimitiveComponent.SetMaterial` _mesh 0 "/Game/Materials/YellowStuff1_Mat.YellowStuff1_Mat" :!label _label)
  (`KismetSystemLibrary.Delay` 0.2)
  (`PrimitiveComponent.SetMaterial` _mesh 0 "/Game/Materials/YellowStuff2_Mat.YellowStuff2_Mat")
  (`KismetSystemLibrary.Delay` 0.2)
  (`PrimitiveComponent.SetMaterial` _mesh 0 "/Game/Materials/YellowStuff3_Mat.YellowStuff3_Mat")
  (`KismetSystemLibrary.Delay` 0.2)
  (`PrimitiveComponent.SetMaterial` _mesh 0 "/Game/Materials/YellowStuff4_Mat.YellowStuff4_Mat")
  (`KismetSystemLibrary.Delay` 0.2)
  (`PrimitiveComponent.SetMaterial` _mesh 0 "/Game/Materials/YellowStuff3_Mat.YellowStuff3_Mat")
  (`KismetSystemLibrary.Delay` 0.2)
  (`PrimitiveComponent.SetMaterial` _mesh 0 "/Game/Materials/YellowStuff2_Mat.YellowStuff2_Mat")
  (`KismetSystemLibrary.Delay` 0.2)
  (goto _label))

(event `self.Box.OnComponentBeginOverlap`
  (params (OverlappedComponent :type "PrimitiveComponent Object Reference") (OtherActor :type "Actor Object Reference") (OtherComp :type "PrimitiveComponent Object Reference") (OtherBodyIndex :type Integer) (bFromSweep :type Boolean) (SweepResult :type "HitResult Structure (by ref)"))
  (`self.K2_DestroyActor`))

(fn `UserConstructionScript`)