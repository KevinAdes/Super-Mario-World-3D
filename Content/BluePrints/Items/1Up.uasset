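; 1-Up pickup Character that roams the level, calling Collect1up on BP_Mario and destroying itself on overlap.
; BlockSpawn raises it gradually with gravity off and query-only collision, using a per-tick loop macro, then restores both and starts movement.
; Tick feeds MovementVector as movement input; wall hits mirror it with random jitter and turn the actor, debounced by a resetting DoOnce.
; A Launch event adds an upward impulse.
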(event `self.ReceiveBeginPlay`
  (set `self.MovementVector` (`self.GetActorForwardVector`))
  (if (`self.StartMoving`)
    (`self.Start Moving`)))

(event `Launch`
  (`CharacterMovementComponent.AddImpulse` (`self.CharacterMovement`) (0.0 0.0 3220.0) true))

(event `self.ReceiveTick`
  (params (DeltaSeconds :type "Float (single-precision)"))
  (`self.AddMovementInput` (`self.MovementVector`) (`CharacterMovementComponent.MaxWalkSpeed` (`self.CharacterMovement`))))

(event `Start Moving`
  (set `CharacterMovementComponent.MaxWalkSpeed` 698.0 (`self.CharacterMovement`)))

(event `BlockSpawn`
  (bind (_returnvalue_x _returnvalue_y _returnvalue_z) (`KismetMathLibrary.BreakVector` (`self.K2_GetActorLocation`)))
  (bind _charactermovement (`self.CharacterMovement`))
  (`PrimitiveComponent.SetCollisionEnabled` (`self.CapsuleComponent`) "QueryOnly")
  (set `CharacterMovementComponent.GravityScale` 0.0 _charactermovement)
  (`self.Custom Loop` 0 12
    (:`Loop Body`
      (`self.K2_SetActorLocation` (`KismetMathLibrary.MakeVector` _returnvalue_x _returnvalue_y (+ _returnvalue_z 10.0))))
    (:`Then 1`
      (`self.Start Moving`)
      (set `CharacterMovementComponent.GravityScale` 6.7 _charactermovement)
      (`PrimitiveComponent.SetCollisionEnabled` (`self.CapsuleComponent`) "QueryAndPhysics"))))

(event `self.CapsuleComponent.OnComponentBeginOverlap`
  (params (OverlappedComponent :type "PrimitiveComponent Object Reference") (OtherActor :type "Actor Object Reference") (OtherComp :type "PrimitiveComponent Object Reference") (OtherBodyIndex :type Integer) (bFromSweep :type Boolean) (SweepResult :type "HitResult Structure (by ref)"))
  (bind _asbp_mario (cast `/Game/BluePrints/BP_Mario` OtherActor))
  (`/Game/BluePrints/BP_Mario.Collect 1up` _asbp_mario)
  (`self.K2_DestroyActor`))

(event `self.CapsuleComponent.OnComponentHit`
  (params (HitComponent :type "PrimitiveComponent Object Reference") (OtherActor :type "Actor Object Reference") (OtherComp :type "PrimitiveComponent Object Reference") (NormalImpulse :type "Vector Structure") (Hit :type "HitResult Structure (by ref)"))
  (bind (_bblockinghit _binitialoverlap _time _distance _location _impactpoint _normal _impactnormal) (`GameplayStatics.BreakHitResult` Hit))
  (bind _returnvalue (`KismetMathLibrary.RandomFloatInRange` -0.5 0.5))
  (bind _returnvalue_2 (`self.K2_GetActorLocation`))
  (if (>= (`KismetMathLibrary.Round` (`KismetMathLibrary.DegAcos` (`KismetMathLibrary.Dot_VectorVector` _impactnormal (0.0 0.0 1.0)))) 90)
    (`/Engine/EditorBlueprintResources/StandardMacros.DoOnce` false :!label _label
      (:`Completed`
        (bind _output_get (set `self.MovementVector` (`KismetMathLibrary.Normal` (+ (`KismetMathLibrary.MirrorVectorByNormal` (`self.MovementVector`) (`KismetMathLibrary.MakeVector` (.x _normal) (.y _normal))) (`KismetMathLibrary.MakeVector` _returnvalue _returnvalue)))))
        (`self.K2_SetActorRotation` (`KismetMathLibrary.FindLookAtRotation` _returnvalue_2 (+ _returnvalue_2 _output_get)))
        (`KismetSystemLibrary.Delay` 0.2)
        (goto _label :!via `Reset`)))))

(fn `UserConstructionScript`)