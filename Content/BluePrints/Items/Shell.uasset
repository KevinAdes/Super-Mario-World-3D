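; Mario-style red Koopa shell character that Mario can stomp, pick up, kick, launch, drop or destroy with a spin jump.
; A state enum drives hit and stomp responses: kicked shells kill Mario on contact, reflect off Wall-tagged actors, and shell collisions destroy one or both.
; Tick moves kicked shells while swapping meshes to fake spinning, and settles thrown shells once slow.
; Kick, Launch and Drop briefly ignore collision with the instigator.
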(event `self.CapsuleComponent.OnComponentHit`
  (params (HitComponent :type "PrimitiveComponent Object Reference") (OtherActor :type "Actor Object Reference") (OtherComp :type "PrimitiveComponent Object Reference") (NormalImpulse :type "Vector Structure") (Hit :type "HitResult Structure (by ref)"))
  (bind (_bblockinghit _binitialoverlap _time _distance _location _impactpoint _normal) (`GameplayStatics.BreakHitResult` Hit))
  (bind (_bblockinghit_2 _binitialoverlap_2 _time_2 _distance_2 _location_2 _impactpoint_2 _normal_2 _impactnormal) (`GameplayStatics.BreakHitResult` Hit))
  (bind _returnvalue (`self.K2_GetActorLocation`))
  (bind _as_mario (`self.As Mario`))
  (bind _as_mario_2 (`self.As Mario`))
  (bind _as_mario_3 (`self.As Mario`))
  (bind _asmario (cast `/Game/BluePrints/Mario` OtherActor)
    (:`then`
      (bind _output_get (set `self.As Mario` _asmario))
      (switch `/Game/BluePrints/Enums/EHoldStates` (`self.States`)
        (:`NewEnumerator0`
          (if (`/Game/BluePrints/Mario.SpinJumping` _output_get) :!label _label
            (`self.K2_DestroyActor`)
            (elif (`/Game/BluePrints/Mario.runheld` _as_mario_3)
              (if (`/Game/BluePrints/Mario.Holding` _as_mario_3)
                (set `self.Impact Normal` (`KismetMathLibrary.MakeVector` (.x _impactnormal) (.y _impactnormal)) :!label _label_2)
                (`PrimitiveComponent.IgnoreActorWhenMoving` (`Character.CapsuleComponent` _as_mario_2) self true)
                (`self.Kick` _as_mario_2)
                (else
                  (`PrimitiveComponent.IgnoreActorWhenMoving` (`Character.CapsuleComponent` _as_mario_3) self true)
                  (`/Game/BluePrints/Mario.Hold` _as_mario_3 self (`self.CapsuleComponent`) (`self.CharacterMovement`))
                  (set `self.States` "NewEnumerator3")))
              (else
                (goto _label_2)))))
        (:`NewEnumerator1`
          (if (`/Game/BluePrints/Mario.SpinJumping` _as_mario)
            (`self.K2_DestroyActor`)
            (else
              (`/Game/BluePrints/Mario.Kill` _as_mario))))
        (:`NewEnumerator2`
          (goto _label))
        (:`NewEnumerator4`
          (goto _label))))
    (:`CastFailed`
      (bind _asshell (cast `/Game/BluePrints/Items/Shell` OtherActor)
        (:`then`
          (switch `/Game/BluePrints/Enums/EHoldStates` (`self.States`)
            (:`NewEnumerator0`
              (bind _states (`/Game/BluePrints/Items/Shell.States` _asshell))
              (switch `/Game/BluePrints/Enums/EHoldStates` _states
                (:`NewEnumerator1`
                  _)
                (:`NewEnumerator3`
                  (`self.K2_DestroyActor` _asshell))
                (:`NewEnumerator2`
                  _)
                (:`NewEnumerator4`
                  _))
              (`self.K2_DestroyActor`))
            (:`NewEnumerator1`
              (switch `/Game/BluePrints/Enums/EHoldStates` _states
                (:`NewEnumerator1`
                  _)
                (:`NewEnumerator3`
                  _)
                (:`NewEnumerator2`
                  _)
                (:`NewEnumerator4`
                  _))
              (`self.K2_DestroyActor` _asshell :!label _label_3)
              (`self.K2_DestroyActor`))
            (:`NewEnumerator2`
              (switch `/Game/BluePrints/Enums/EHoldStates` _states :!label _label_4
                (:`NewEnumerator3`
                  (goto _label_3))
                (:`NewEnumerator2`
                  (goto _label_3))
                (:`NewEnumerator4`
                  (goto _label_3))))
            (:`NewEnumerator4`
              (goto _label_4))))
        (:`CastFailed`
          (if (`self.ActorHasTag` OtherActor "Wall")
            (bind _output_get_2 (set `self.Impact Normal` (`KismetMathLibrary.MirrorVectorByNormal` (`self.Impact Normal`) (`KismetMathLibrary.MakeVector` (.x _normal) (.y _normal)))))
            (`self.K2_SetActorRotation` (`KismetMathLibrary.FindLookAtRotation` _returnvalue (+ _returnvalue _output_get_2)))))))))

(event `self.ReceiveTick`
  (params (DeltaSeconds :type "Float (single-precision)"))
  (bind _mesh (`self.Mesh`))
  (bind _returnvalue (`|EnumEquality` (`self.States`) "NewEnumerator1"))
  (bind _returnvalue_2 (`|EnumEquality` (`self.States`) "NewEnumerator1"))
  (switch `/Game/BluePrints/Enums/EHoldStates` (`self.States`)
    (:`NewEnumerator1`
      (`self.AddMovementInput` (`self.Impact Normal`))
      (if (not (`self.Moving`))
        (set `self.Moving` true))
      (`SkinnedMeshComponent.SetSkinnedAssetAndUpdate` _mesh "/Game/Models/Koopa/Red/Shell/RedShell34.RedShell34" true :!label _label_5)
      (`self.Delay4`
        (:`Completed`
          (if _returnvalue_2
            (`SkinnedMeshComponent.SetSkinnedAssetAndUpdate` _mesh "/Game/Models/Koopa/Red/Shell/RedShellSide.RedShellSide" true)
            (`self.Delay4`
              (:`Completed`
                (if _returnvalue_2
                  (`SkinnedMeshComponent.SetSkinnedAssetAndUpdate` _mesh "/Game/Models/Koopa/Red/Shell/RedShell342.RedShell342" true)
                  (`self.Delay4`
                    (:`Completed`
                      (if _returnvalue
                        (`SkinnedMeshComponent.SetSkinnedAssetAndUpdate` _mesh "/Game/Models/Koopa/Red/Shell/RedShellFront.RedShellFront" true)
                        (`self.Delay4`
                          (:`Completed`
                            (if _returnvalue
                              (goto _label_5)
                              (else
                                _)))))))))))
          (`SkinnedMeshComponent.SetSkinnedAssetAndUpdate` (`self.Mesh`) "/Game/Models/Koopa/Red/Shell/RedShellSide.RedShellSide" true))))
    (:`NewEnumerator2`
      (if (< (`KismetMathLibrary.VSize` (`CharacterMovementComponent.GetLastUpdateVelocity` (`self.CharacterMovement`))) 10.0) :!label _label_6
        (set `self.States` "NewEnumerator0")))
    (:`NewEnumerator4`
      (goto _label_6))))

(event `self.StompBox.OnComponentBeginOverlap`
  (params (OverlappedComponent :type "PrimitiveComponent Object Reference") (OtherActor :type "Actor Object Reference") (OtherComp :type "PrimitiveComponent Object Reference") (OtherBodyIndex :type Integer) (bFromSweep :type Boolean) (SweepResult :type "HitResult Structure (by ref)"))
  (bind _as_mario (`self.As Mario`))
  (bind _asmario (cast `/Game/BluePrints/Mario` OtherActor))
  (set `self.As Mario` _asmario)
  (if (== (`/Game/BluePrints/Mario.Shoebox` _asmario) OtherComp)
    (if (`/Game/BluePrints/Mario.SpinJumping` (`self.As Mario`))
      (`self.K2_DestroyActor`)
      (elif (`self.Moving`)
        (`SkinnedMeshComponent.SetSkinnedAssetAndUpdate` (`self.Mesh`) "/Game/Models/Koopa/Red/Shell/RedShellFront.RedShellFront" false)
        (set `self.States` "NewEnumerator0")
        (set `self.Moving` false)
        (`self.CalcMarioJump`)
        (elif (`/Game/BluePrints/Mario.runheld` _as_mario)
          (if (`/Game/BluePrints/Mario.Holding` _as_mario)
            (`self.Calculate MoveVector` (`self.As Mario`) :!label _label_7)
            (`self.CalcMarioJump`)
            (else
              (`PrimitiveComponent.IgnoreActorWhenMoving` (`Character.CapsuleComponent` _as_mario) self true)
              (`/Game/BluePrints/Mario.Hold` _as_mario self (`self.CapsuleComponent`) (`self.CharacterMovement`))
              (set `self.States` "NewEnumerator3")))
          (else
            (goto _label_7)))))))

(event `Kick`
  (params (Kicker :type "Actor Object Reference"))
  (bind _charactermovement (`self.CharacterMovement`))
  (`PrimitiveComponent.IgnoreActorWhenMoving` (`self.CapsuleComponent`) Kicker true)
  (set `self.States` "NewEnumerator1")
  (set `CharacterMovementComponent.GravityScale` 6.8 _charactermovement)
  (set `MovementComponent.Velocity` (0.0 0.0 0.0) _charactermovement)
  (`KismetSystemLibrary.Delay` 0.5)
  (`PrimitiveComponent.IgnoreActorWhenMoving` (`self.CapsuleComponent`) Kicker false)
  (`PrimitiveComponent.IgnoreActorWhenMoving` (`self.GetComponentByClass` Kicker "/Script/Engine.CapsuleComponent") self false))

(event `Launch`
  (params (Launcher :type "Actor Object Reference"))
  (bind _charactermovement (`self.CharacterMovement`))
  (bind (_launch_velocity_x _launch_velocity_y) (`KismetMathLibrary.BreakVector` (`self.Launch Velocity`)))
  (bind _charactermovement_2 (`self.CharacterMovement`))
  (bind (_returnvalue_x _returnvalue_y) (`KismetMathLibrary.BreakVector` (`CharacterMovementComponent.GetLastUpdateVelocity` _charactermovement_2)))
  (`PrimitiveComponent.IgnoreActorWhenMoving` (`self.CapsuleComponent`) Launcher true)
  (set `self.States` "NewEnumerator2")
  (set `CharacterMovementComponent.GravityScale` 6.8 _charactermovement)
  (`CharacterMovementComponent.AddImpulse` _charactermovement (`KismetMathLibrary.MakeVector` _launch_velocity_x _launch_velocity_y 4210.0) true)
  (`KismetSystemLibrary.Delay` 0.2)
  (`PrimitiveComponent.IgnoreActorWhenMoving` (`self.CapsuleComponent`) Launcher false)
  (`PrimitiveComponent.IgnoreActorWhenMoving` (`self.GetComponentByClass` Launcher "/Script/Engine.CapsuleComponent") self false)
  (`KismetSystemLibrary.Delay` 0.8)
  (set `CharacterMovementComponent.GravityScale` 0.0 _charactermovement_2)
  (set `MovementComponent.Velocity` (`KismetMathLibrary.MakeVector` _returnvalue_x _returnvalue_y -2380.0) _charactermovement_2))

(event `Drop`
  (params (Dropper :type "Actor Object Reference"))
  (bind _charactermovement (`self.CharacterMovement`))
  (bind (_launch_velocity_x _launch_velocity_y) (`KismetMathLibrary.BreakVector` (`self.Launch Velocity`)))
  (`PrimitiveComponent.IgnoreActorWhenMoving` (`self.CapsuleComponent`) Dropper true)
  (set `self.States` "NewEnumerator4")
  (set `CharacterMovementComponent.GravityScale` 6.8 _charactermovement)
  (`CharacterMovementComponent.AddImpulse` _charactermovement (`KismetMathLibrary.MakeVector` _launch_velocity_x _launch_velocity_y) true)
  (`KismetSystemLibrary.Delay` 0.15)
  (`PrimitiveComponent.IgnoreActorWhenMoving` (`self.CapsuleComponent`) Dropper false)
  (`PrimitiveComponent.IgnoreActorWhenMoving` (`self.GetComponentByClass` Dropper "/Script/Engine.CapsuleComponent") self false))

(fn `Calculate MoveVector`
  (params (Kicker :type "Actor Object Reference"))
  (bind (_returnvalue_x _returnvalue_y) (`KismetMathLibrary.BreakVector` (- (`self.K2_GetActorLocation` self) (`self.K2_GetActorLocation` Kicker))))
  (set `self.Impact Normal` (`KismetMathLibrary.MakeVector` _returnvalue_x _returnvalue_y))
  (`self.Kick` Kicker))

(fn `UserConstructionScript`)