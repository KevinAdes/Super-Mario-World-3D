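; Collectible coin item for a Mario-style game, picked up when BP_Mario touches it.
; BeginPlay loops endlessly, cycling four static meshes on short delays as a flipbook-style animation.
; Mesh overlap calls CollectCoin on Mario, then the coin's own CollectCoin spawns a Niagara sparkle at its location and destroys the actor.
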(event `self.ReceiveBeginPlay`
  (bind _staticmesh (`self.StaticMesh`))
  (`StaticMeshComponent.SetStaticMesh` _staticmesh "/Game/Models/Items/Coin1.Coin1" :!label _label)
  (`KismetSystemLibrary.Delay` 0.15)
  (`StaticMeshComponent.SetStaticMesh` _staticmesh "/Game/Models/Items/Coin2.Coin2")
  (`KismetSystemLibrary.Delay` 0.15)
  (`StaticMeshComponent.SetStaticMesh` _staticmesh "/Game/Models/Items/Coin3.Coin3")
  (`KismetSystemLibrary.Delay` 0.15)
  (`StaticMeshComponent.SetStaticMesh` _staticmesh "/Game/Models/Items/Coin4.Coin4")
  (`KismetSystemLibrary.Delay` 0.15)
  (goto _label))

(event `self.StaticMesh.OnComponentBeginOverlap`
  (params (OverlappedComponent :type "PrimitiveComponent Object Reference") (OtherActor :type "Actor Object Reference") (OtherComp :type "PrimitiveComponent Object Reference") (OtherBodyIndex :type Integer) (bFromSweep :type Boolean) (SweepResult :type "HitResult Structure (by ref)"))
  (bind _asbp_mario (cast `/Game/BluePrints/BP_Mario` OtherActor))
  (`/Game/BluePrints/BP_Mario.Collect Coin` _asbp_mario)
  (`self.CollectCoin`))

(fn `CollectCoin`
  (`NiagaraFunctionLibrary.SpawnSystemAtLocation` "/Game/Particles/Systems/NS_Sparkle.NS_Sparkle" (`self.K2_GetActorLocation`) (struct) (1.0 1.0 1.0) false)
  (`self.K2_DestroyActor`))

(fn `UserConstructionScript`)