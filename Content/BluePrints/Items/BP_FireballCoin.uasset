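; BP_FireballCoin is a moving coin pickup that falls, bounces off walls and awards points to BP_Mario when collected.
; Each tick it applies capped gravity to MovementVector, then sweeps its location, retrying horizontally when blocked.
; If that also fails, it mirrors movement around the flattened impact normal.
; CollectCoin spawns a Niagara points popup and adds score before calling the parent logic.
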(event `self.ReceiveTick`
  (params (DeltaSeconds :type "Float (single-precision)"))
  (`parent.ReceiveTick` DeltaSeconds)
  (`|ExecutionSequence`
    (:`then_0`
      (`self.ApplyGravity`))
    (:`then_1`
      (`self.UpdateLocation`))))

(fn `ApplyGravity`
  (bind (_movementvector_x _movementvector_y _movementvector_z) (`KismetMathLibrary.BreakVector` (`self.MovementVector`)))
  (if (<= _movementvector_z -24.0)
    (set `self.MovementVector` (`KismetMathLibrary.MakeVector` _movementvector_x _movementvector_y -24.0))
    (else
      (set `self.MovementVector` (`KismetMathLibrary.MakeVector` _movementvector_x _movementvector_y (- _movementvector_z 0.375))))))

(fn `CollectCoin`
  (bind _returnvalue (`NiagaraFunctionLibrary.SpawnSystemAtLocation` "/Game/Particles/Systems/NS_Points.NS_Points" (`self.K2_GetActorLocation`)))
  (`FXSystemComponent.SetIntParameter` _returnvalue "Particles_MeshIndex" 2)
  (`FXSystemComponent.SetIntParameter` _returnvalue "Particles_MeshIndex001" 1)
  (bind _returnvalue_2 (`GameplayStatics.GetActorOfClass` "/Game/BluePrints/BP_Mario.BP_Mario_C"))
  (`/Game/BluePrints/BP_Mario.AwardPoints` _returnvalue_2 200 false)
  (`parent.CollectCoin`))

(fn `FlipMovement`
  (params (InVec :type "Vector Structure"))
  (set `self.MovementVector` (`KismetMathLibrary.MirrorVectorByNormal` (`self.MovementVector`) (`KismetMathLibrary.MakeVector` (.x InVec) (.y InVec)))))

(fn `UpdateLocation`
  (bind (_movementvector_x _movementvector_y) (`KismetMathLibrary.BreakVector` (`self.MovementVector`)))
  (bind (_sweephitresult _returnvalue) (`self.K2_SetActorLocation` (+ (`self.K2_GetActorLocation`) (`self.MovementVector`)) true))
  (if (not _returnvalue)
    (bind (_sweephitresult_2 _returnvalue_2) (`self.K2_SetActorLocation` (+ (`self.K2_GetActorLocation`) (`KismetMathLibrary.MakeVector` _movementvector_x _movementvector_y)) true))
    (if (not _returnvalue_2)
      (`self.FlipMovement` (`.ImpactNormal` (`GameplayStatics.BreakHitResult` _sweephitresult_2))))))

(fn `UserConstructionScript`
  (`parent.UserConstructionScript`))