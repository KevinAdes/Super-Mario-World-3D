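; Mushroom power-up Character that moves by per-tick location offsets and, on overlapping BP_Mario, grants a power-up and destroys itself.
; BlockSpawn raises it with a frame-delayed loop macro, gravity off and collision query-only, then starts forward movement.
; Wall hits mirror its direction with random jitter, debounced by a delayed DoOnce.
; Launch pops it upward; ItemBoxFall drifts it down overlapping only one channel, with a looping timer.
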(event `Launch`
  (`CharacterMovementComponent.AddImpulse` (`self.CharacterMovement`) (0.0 0.0 3220.0) true))

(event `Start Moving`
  (set `self.MovementVector` (`self.GetActorForwardVector`)))

(event `self.ReceiveTick`
  (params (DeltaSeconds :type "Float (single-precision)"))
  (`self.K2_SetActorLocation` (+ (`self.K2_GetActorLocation`) (* (`self.MovementVector`) 10))))

(event `BlockSpawn`
  (bind (_returnvalue_x _returnvalue_y _returnvalue_z) (`KismetMathLibrary.BreakVector` (`self.K2_GetActorLocation`)))
  (`PrimitiveComponent.SetCollisionEnabled` (`self.CapsuleComponent`) "QueryOnly")
  (set `CharacterMovementComponent.GravityScale` 0.0 (`self.CharacterMovement`))
  (`self.Custom Loop` 0 12
    (:`Loop Body`
      (`self.K2_SetActorLocation` (`KismetMathLibrary.MakeVector` _returnvalue_x _returnvalue_y (+ _returnvalue_z 10.0))))
    (:`Then 1`
      (`self.Start Moving`)
      (set `CharacterMovementComponent.GravityScale` 6.7 (`self.CharacterMovement`))
      (`PrimitiveComponent.SetCollisionEnabled` (`self.CapsuleComponent`) "QueryAndPhysics"))))

(event `self.CapsuleComponent.OnComponentBeginOverlap`
  (params (OverlappedComponent :type "PrimitiveComponent Object Reference") (OtherActor :type "Actor Object Reference") (OtherComp :type "PrimitiveComponent Object Reference") (OtherBodyIndex :type Integer) (bFromSweep :type Boolean) (SweepResult :type "HitResult Structure (by ref)"))
  (bind _asbp_mario (cast `/Game/BluePrints/BP_Mario` OtherActor))
  (`/Game/BluePrints/BP_Mario.CollectPowerUp` _asbp_mario 1)
  (`self.K2_DestroyActor`))

(event `self.CapsuleComponent.OnComponentHit`
  (params (HitComponent :type "PrimitiveComponent Object Reference") (OtherActor :type "Actor Object Reference") (OtherComp :type "PrimitiveComponent Object Reference") (NormalImpulse :type "Vector Structure") (Hit :type "HitResult Structure (by ref)"))
  (bind (_bblockinghit _binitialoverlap _time _distance _location _impactpoint _normal _impactnormal) (`GameplayStatics.BreakHitResult` Hit))
  (bind _returnvalue (`KismetMathLibrary.RandomFloatInRange` -0.5 0.5))
  (bind _returnvalue_2 (`self.K2_GetActorLocation`))
  (if (>= (`KismetMathLibrary.Round` (`KismetMathLibrary.DegAcos` (`KismetMathLibrary.Dot_VectorVector` _impactnormal (0.0 0.0 1.0)))) 90)
    (`/Engine/EditorBlueprintResources/StandardMacros.DoOnce` false :!label _label
      (:`Completed`
        (bind _output_get (set `self.MovementVector` (`KismetMathLibrary.Normal` (+ (`KismetMathLibrary.MirrorVectorByNormal` (`self.MovementVector`) (`KismetMathLibrary.MakeVector` (.x _normal) (.y _normal))) (`KismetMathLibrary.MakeVector` _returnvalue _returnvalue)))))
        (`self.K2_SetActorRotation` (`KismetMathLibrary.FindLookAtRotation` _returnvalue_2 (+ _returnvalue_2 _output_get)))
        (`KismetSystemLibrary.Delay` 0.2)
        (goto _label :!via `Reset`)))))

(fn `ItemBoxFall`
  (bind _capsulecomponent (`self.CapsuleComponent`))
  (`KismetSystemLibrary.K2_SetTimerDelegate` (`|CreateDelegate` :!event `ToggleOpacity`) 0.3 true)
  (set `self.MovementVector` (0.0 0.0 -0.5))
  (set `CharacterMovementComponent.GravityScale` 0.0 (`self.CharacterMovement`))
  (`PrimitiveComponent.SetCollisionResponseToAllChannels` _capsulecomponent "ECR_Ignore")
  (`PrimitiveComponent.SetCollisionResponseToChannel` _capsulecomponent "ECC_GameTraceChannel1" "ECR_Overlap"))

(fn `ToggleOpacity`
  (bind _staticmesh (`self.StaticMesh`))
  (`SceneComponent.SetVisibility` _staticmesh (not (`SceneComponent.bVisible` _staticmesh)) false))

(fn `UserConstructionScript`)