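; BP_FireFlower is a character-based fire flower pickup that calls CollectPowerUp on an overlapping BP_Mario, then destroys itself.
; BlockSpawn raises it in small per-tick steps with gravity off and query-only collision, using a delayed-loop macro, then restores gravity and physics collision.
; Launch applies an upward impulse, and Flip mirrors the mesh on X.
; BeginPlay starts a short one-shot timer.
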(event `self.ReceiveBeginPlay`
  (`KismetSystemLibrary.K2_SetTimerDelegate` (`|CreateDelegate` :!event `Flip`) 0.2))

(event `Launch`
  (`CharacterMovementComponent.AddImpulse` (`self.CharacterMovement`) (0.0 0.0 3220.0) true))

(event `BlockSpawn`
  (bind (_returnvalue_x _returnvalue_y _returnvalue_z) (`KismetMathLibrary.BreakVector` (`self.K2_GetActorLocation`)))
  (`PrimitiveComponent.SetCollisionEnabled` (`self.CapsuleComponent`) "QueryOnly")
  (set `CharacterMovementComponent.GravityScale` 0.0 (`self.CharacterMovement`))
  (`self.Custom Loop` 0 12
    (:`Loop Body`
      (`self.K2_SetActorLocation` (`KismetMathLibrary.MakeVector` _returnvalue_x _returnvalue_y (+ _returnvalue_z 10.0))))
    (:`Then 1`
      (set `CharacterMovementComponent.GravityScale` 6.7 (`self.CharacterMovement`))
      (`PrimitiveComponent.SetCollisionEnabled` (`self.CapsuleComponent`) "QueryAndPhysics"))))

(event `self.CapsuleComponent.OnComponentBeginOverlap`
  (params (OverlappedComponent :type "PrimitiveComponent Object Reference") (OtherActor :type "Actor Object Reference") (OtherComp :type "PrimitiveComponent Object Reference") (OtherBodyIndex :type Integer) (bFromSweep :type Boolean) (SweepResult :type "HitResult Structure (by ref)"))
  (bind _asbp_mario (cast `/Game/BluePrints/BP_Mario` OtherActor))
  (`/Game/BluePrints/BP_Mario.CollectPowerUp` _asbp_mario 2)
  (`self.K2_DestroyActor`))

(fn `Flip`
  (bind _staticmesh (`self.StaticMesh`))
  (bind (_relativescale3d_x _relativescale3d_y _relativescale3d_z) (`KismetMathLibrary.BreakVector` (`SceneComponent.RelativeScale3D` _staticmesh)))
  (`SceneComponent.SetRelativeScale3D` _staticmesh (`KismetMathLibrary.MakeVector` (* _relativescale3d_x -1.0) _relativescale3d_y _relativescale3d_z)))

(fn `UserConstructionScript`)