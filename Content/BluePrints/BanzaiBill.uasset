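; Banzai Bill enemy that flies toward Mario, destroys him on body contact and can be stomped.
; It takes an initial heading to Mario at BeginPlay, PawnSensing updates the target heading, and Tick drives rotation and movement along a fixed-alpha blend of both.
; Stomp boxes use JumpCheck to match Mario's Shoebox, then bounce him with gravity and impulse based on held jump, and destroy the Bill.
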(event `self.ReceiveBeginPlay`
  (bind _returnvalue (`GameplayStatics.GetActorOfClass` "/Game/BluePrints/Mario.Mario_C"))
  (bind (_returnvalue_x _returnvalue_y) (`KismetMathLibrary.BreakVector` (- (`self.K2_GetActorLocation` _returnvalue) (`self.K2_GetActorLocation` self))))
  (bind _output_get (set `self.Move Vector` (`KismetMathLibrary.MakeVector` _returnvalue_x _returnvalue_y)))
  (set `self.Vector to lerp to` _output_get)
  (`self.SetActorTickEnabled` true))

(event `self.PawnSensing.OnSeePawn`
  (params (Pawn :type "Pawn Object Reference"))
  (bind _asmario (cast `/Game/BluePrints/Mario` Pawn))
  (bind (_returnvalue_x _returnvalue_y) (`KismetMathLibrary.BreakVector` (- (`self.K2_GetActorLocation` _asmario) (`self.K2_GetActorLocation` self))))
  (set `self.Vector to lerp to` (`KismetMathLibrary.MakeVector` _returnvalue_x _returnvalue_y)))

(event `self.ReceiveTick`
  (params (DeltaSeconds :type "Float (single-precision)"))
  (bind _returnvalue (`KismetMathLibrary.VLerp` (`self.Move Vector`) (`self.Vector to lerp to`) 0.8))
  (`self.K2_SetActorRotation` (`KismetMathLibrary.Conv_VectorToRotator` _returnvalue))
  (`self.AddMovementInput` _returnvalue 1.0 true))

(event `self.Capsule.OnComponentBeginOverlap`
  (params (OverlappedComponent :type "PrimitiveComponent Object Reference") (OtherActor :type "Actor Object Reference") (OtherComp :type "PrimitiveComponent Object Reference") (OtherBodyIndex :type Integer) (bFromSweep :type Boolean) (SweepResult :type "HitResult Structure (by ref)"))
  (bind _asmario (cast `/Game/BluePrints/Mario` OtherActor))
  (`self.K2_DestroyActor` _asmario))

(event `self.Cylinder.OnComponentBeginOverlap`
  (params (OverlappedComponent :type "PrimitiveComponent Object Reference") (OtherActor :type "Actor Object Reference") (OtherComp :type "PrimitiveComponent Object Reference") (OtherBodyIndex :type Integer) (bFromSweep :type Boolean) (SweepResult :type "HitResult Structure (by ref)"))
  (bind _asmario (cast `/Game/BluePrints/Mario` OtherActor))
  (`self.K2_DestroyActor` _asmario))

(event `self.Capsule1.OnComponentBeginOverlap`
  (params (OverlappedComponent :type "PrimitiveComponent Object Reference") (OtherActor :type "Actor Object Reference") (OtherComp :type "PrimitiveComponent Object Reference") (OtherBodyIndex :type Integer) (bFromSweep :type Boolean) (SweepResult :type "HitResult Structure (by ref)"))
  (bind _asmario (cast `/Game/BluePrints/Mario` OtherActor))
  (`self.K2_DestroyActor` _asmario))

(event `self.StompBox.OnComponentBeginOverlap`
  (params (OverlappedComponent :type "PrimitiveComponent Object Reference") (OtherActor :type "Actor Object Reference") (OtherComp :type "PrimitiveComponent Object Reference") (OtherBodyIndex :type Integer) (bFromSweep :type Boolean) (SweepResult :type "HitResult Structure (by ref)"))
  (bind _as_mario (`self.As Mario`))
  (bind _as_mario_2 (`self.As Mario`))
  (bind _charactermovement (`Character.CharacterMovement` _as_mario))
  (bind _charactermovement_2 (`Character.CharacterMovement` _as_mario_2))
  (`self.JumpCheck` OtherActor OtherComp
    (:`then`
      (`/Engine/EditorBlueprintResources/StandardMacros.DoOnce` false :!label _label
        (:`Completed`
          (set `CharacterMovementComponent.JumpZVelocity` 0.0 _charactermovement)
          (set `MovementComponent.Velocity` (0.0 0.0 0.0) _charactermovement)
          (if (`/Game/BluePrints/Mario.JumpHeld` _as_mario)
            (set `CharacterMovementComponent.GravityScale` 6.93 _charactermovement)
            (`CharacterMovementComponent.AddImpulse` _charactermovement (0.0 0.0 3000.0) true)
            (else
              (set `CharacterMovementComponent.GravityScale` 16.3 _charactermovement)
              (`CharacterMovementComponent.AddImpulse` _charactermovement (0.0 0.0 2910.0) true)))
          (`self.K2_DestroyActor`))))
    (:`else`
      (`/Engine/EditorBlueprintResources/StandardMacros.DoOnce` false :!label _label_2
        (:`Completed`
          (set `CharacterMovementComponent.JumpZVelocity` 0.0 _charactermovement_2)
          (set `MovementComponent.Velocity` (0.0 0.0 0.0) _charactermovement_2)
          (if (`/Game/BluePrints/Mario.JumpHeld` _as_mario_2)
            (set `CharacterMovementComponent.GravityScale` 6.93 _charactermovement_2)
            (`CharacterMovementComponent.AddImpulse` _charactermovement_2 (0.0 0.0 3000.0) true)
            (else
              (set `CharacterMovementComponent.GravityScale` 16.3 _charactermovement_2)
              (`CharacterMovementComponent.AddImpulse` _charactermovement_2 (0.0 0.0 2910.0) true)))
          (`self.K2_DestroyActor`))))))

(event `self.StompBox1.OnComponentBeginOverlap`
  (params (OverlappedComponent :type "PrimitiveComponent Object Reference") (OtherActor :type "Actor Object Reference") (OtherComp :type "PrimitiveComponent Object Reference") (OtherBodyIndex :type Integer) (bFromSweep :type Boolean) (SweepResult :type "HitResult Structure (by ref)"))
  (`self.JumpCheck` OtherActor OtherComp
    (:`then`
      (goto _label))
    (:`else`
      (goto _label_2))))

(fn `UserConstructionScript`)