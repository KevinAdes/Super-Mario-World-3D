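; Mario-style spin block that, when hit by a shell or Mario, either spins or spawns its item, depending on BlockType.
; Spinning disables all collision and loops four meshes through chained delays until a timer restores the solid block.
; Item blocks spawn HitItem above, switch to the hit mesh and stay used.
; Without a HitItem, a powered-up, spin-jumping Mario landing on top bounces and destroys the block with particles.
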(event `Spin`
  (set `self.Block Hit` true)
  (`/Engine/EditorBlueprintResources/StandardMacros.DoOnce` false :!label _label
    (:`Completed`
      (`KismetSystemLibrary.K2_SetTimerDelegate` (delegate `Stop Spinning`) 5.0)
      (`PrimitiveComponent.SetCollisionEnabled` (`self.StaticMesh`) "NoCollision")
      (`PrimitiveComponent.SetCollisionEnabled` (`self.StompBox`) "NoCollision")
      (`PrimitiveComponent.SetCollisionEnabled` (`self.Shell Box`) "NoCollision")
      (`PrimitiveComponent.SetCollisionEnabled` (`self.Mario Box`) "NoCollision")
      (set `self.Spinning` true)
      (`StaticMeshComponent.SetStaticMesh` (`self.StaticMesh`) "/Game/Models/Blocks/Spin1.Spin1" :!label _label_2)
      (`KismetSystemLibrary.Delay` 0.2)
      (if (`self.Spinning`)
        (`StaticMeshComponent.SetStaticMesh` (`self.StaticMesh`) "/Game/Models/Blocks/Spin2.Spin2")
        (`KismetSystemLibrary.Delay` 0.2)
        (if (`self.Spinning`)
          (`StaticMeshComponent.SetStaticMesh` (`self.StaticMesh`) "/Game/Models/Blocks/Spin3.Spin3")
          (`KismetSystemLibrary.Delay` 0.2)
          (if (`self.Spinning`)
            (`StaticMeshComponent.SetStaticMesh` (`self.StaticMesh`) "/Game/Models/Blocks/Spin4.Spin4")
            (`KismetSystemLibrary.Delay` 0.2)
            (if (`self.Spinning`)
              (goto _label_2))))))))

(event `Stop Spinning`
  (set `self.Block Hit` false)
  (set `self.Spinning` false)
  (`|ExecutionSequence`
    (:`then_0`
      (goto _label :!via `Reset`))
    (:`then_1`
      (`PrimitiveComponent.SetCollisionEnabled` (`self.StaticMesh`) "QueryAndPhysics")
      (`PrimitiveComponent.SetCollisionEnabled` (`self.StompBox`) "QueryAndPhysics")
      (`PrimitiveComponent.SetCollisionEnabled` (`self.Shell Box`) "QueryAndPhysics")
      (`PrimitiveComponent.SetCollisionEnabled` (`self.Mario Box`) "QueryAndPhysics")
      (`StaticMeshComponent.SetStaticMesh` (`self.StaticMesh`) "/Game/Models/Blocks/SpinNeutral.SpinNeutral"))))

(event `self.StompBox.OnComponentBeginOverlap`
  (params (OverlappedComponent :type "PrimitiveComponent Object Reference") (OtherActor :type "Actor Object Reference") (OtherComp :type "PrimitiveComponent Object Reference") (OtherBodyIndex :type Integer) (bFromSweep :type Boolean) (SweepResult :type "HitResult Structure (by ref)"))
  (if (not (`KismetSystemLibrary.IsValidClass` (`self.Hit Item`)))
    (bind _asbp_mario (cast `/Game/BluePrints/BP_Mario` OtherActor))
    (bind _output_get (set `self.As Mario` _asbp_mario))
    (`Character.StopJumping` _output_get)
    (if (and (`/Game/BluePrints/BP_Mario.SpinJumping` _output_get) (== (`/Game/BluePrints/BP_Mario.Shoebox` _output_get) OtherComp) (> (`/Game/BluePrints/BP_Mario.PowerState` (`self.As Mario`)) 0))
      (`/Game/BluePrints/BP_Mario.BlockBounce` (`self.As Mario`))
      (`NiagaraFunctionLibrary.SpawnSystemAtLocation` "/Game/Particles/Systems/NS_BlockBreakParticle.NS_BlockBreakParticle" (`self.K2_GetActorLocation`))
      (`self.K2_DestroyActor`))))

(event `self.Shell Box.OnComponentHit`
  (params (HitComponent :type "PrimitiveComponent Object Reference") (OtherActor :type "Actor Object Reference") (OtherComp :type "PrimitiveComponent Object Reference") (NormalImpulse :type "Vector Structure") (Hit :type "HitResult Structure (by ref)"))
  (`self.HandleBlockHit`))

(event `self.Mario Box.OnComponentHit`
  (params (HitComponent :type "PrimitiveComponent Object Reference") (OtherActor :type "Actor Object Reference") (OtherComp :type "PrimitiveComponent Object Reference") (NormalImpulse :type "Vector Structure") (Hit :type "HitResult Structure (by ref)"))
  (bind _asbp_mario (cast `/Game/BluePrints/BP_Mario` OtherActor))
  (if (`|EnumEquality` (`/Game/BluePrints/BP_Mario.MarioStates` _asbp_mario) "NewEnumerator1")
    (`/Game/BluePrints/BP_Mario.UpdateVerticalVelocity` _asbp_mario -4.0)
    (`self.HandleBlockHit`)))

(fn `HandleBlockHit`
  (if (not (`self.Block Hit`))
    (switch `/Game/BluePrints/Enums/ESpinBlockTypes` (`self.BlockType`)
      (:`NewEnumerator0`
        (`self.Spin`))
      (:`NewEnumerator1`
        (`self.SpawnItem`)))))

(fn `SpawnItem`
  (bind _returnvalue (`self.GetTransform`))
  (bind _returnvalue_2 (`|SpawnActorFromClass` (`self.Hit Item`) (`KismetMathLibrary.MakeTransform` (`KismetMathLibrary.MakeVector` (.x (.location _returnvalue)) (.y (.location _returnvalue)) (+ (.z (.location _returnvalue)) 40.0)) (.rotation _returnvalue) (.scale _returnvalue)) "AlwaysSpawn" "SelectDefaultAtRuntime" null null))
  (bind _instigator (`Actor.Instigator` _returnvalue_2))
  (`Pawn.SpawnDefaultController` _instigator)
  (`StaticMeshComponent.SetStaticMesh` (`self.StaticMesh`) "/Game/Models/Blocks/HitBlock.HitBlock")
  (set `self.Block Hit` true)
  (if (== (`self.Hit Item`) "/Game/BluePrints/Items/Mushroom.Mushroom_C")
    (bind _asmushroom (cast `/Game/BluePrints/Items/Mushroom` _instigator))
    (`/Game/BluePrints/Items/Mushroom.BlockSpawn` _asmushroom)
    (elif (== (`self.Hit Item`) "/Game/BluePrints/Items/1Up.1Up_C")
      (bind _as1up (cast `/Game/BluePrints/Items/1Up` _instigator))
      (`/Game/BluePrints/Items/1Up.BlockSpawn` _as1up))))

(fn `UserConstructionScript`)