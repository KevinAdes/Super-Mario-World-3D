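; BP_SpeakerBlock is a message block that shows its text when Mario hits it while moving upward.
; A hit on MarioBox checks Mario's state and upward velocity, then zeroes his vertical velocity.
; The TL_Hit timeline moves the mesh by adding its alpha as a Z offset each update.
; When it finishes, Mario displays the block's Message and the game pauses.
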(event `self.ReceiveBeginPlay`)

(event `self.Mario Box.OnComponentHit`
  (params (HitComponent :type "PrimitiveComponent Object Reference") (OtherActor :type "Actor Object Reference") (OtherComp :type "PrimitiveComponent Object Reference") (NormalImpulse :type "Vector Structure") (Hit :type "HitResult Structure (by ref)"))
  (bind _asbp_mario (cast `/Game/BluePrints/BP_Mario` OtherActor))
  (bind (_velocity_x _velocity_y _velocity_z) (`KismetMathLibrary.BreakVector` (`/Game/BluePrints/BP_Mario.Velocity` _asbp_mario)))
  (if (and (`|EnumEquality` (`/Game/BluePrints/BP_Mario.MarioStates` _asbp_mario) "NewEnumerator1") (> _velocity_z 0.0))
    (`/Game/BluePrints/BP_Mario.UpdateVerticalVelocity` _asbp_mario 0.0)
    (bind (_direction _lerpalpha) (`Timeline|TL_Hit` :!via `PlayFromStart`)
      (:`Update`
        (`SceneComponent.K2_AddRelativeLocation` (`self.StaticMesh`) (`KismetMathLibrary.MakeVector` 0.0 0.0 _lerpalpha) false false))
      (:`Finished`
        (`/Game/BluePrints/BP_Mario.DisplayMessage` _asbp_mario (`self.Message`))
        (`GameplayStatics.SetGamePaused` true)))))

(fn `UserConstructionScript`)