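; Winged variant of a question block that moves along a path until it is hit.
; Each Tick it sweeps its location and yaw to the Path component's reference point, then disables ticking once BlockHit is set.
; The construction script initializes the BPCWings component.
; SetBlockHit destroys both wings and that component before running the parent's hit logic.
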(event `self.ReceiveTick`
  (params (DeltaSeconds :type "Float (single-precision)"))
  (bind _returnvalue (`SceneComponent.K2_GetComponentToWorld` (`/Game/BluePrints/LevelStuff/Path.Reference point` (`self.Path`))))
  (`parent.ReceiveTick` DeltaSeconds)
  (if (`self.BlockHit`)
    (`self.SetActorTickEnabled` false)
    (else
      (`self.K2_SetActorTransform` (`KismetMathLibrary.MakeTransform` (`KismetMathLibrary.MakeVector` (.x (.location _returnvalue)) (.y (.location _returnvalue)) (.z (.location _returnvalue))) (`KismetMathLibrary.MakeRotator` 0.0 0.0 (.yaw (.rotation _returnvalue)))) true))))

(fn `SetBlockHit`
  (`ActorComponent.K2_DestroyComponent` (`/Game/BluePrints/Components/BPC_Wings.RightWing` (`self.BPC_Wings`)))
  (`ActorComponent.K2_DestroyComponent` (`/Game/BluePrints/Components/BPC_Wings.LeftWing` (`self.BPC_Wings`)))
  (`ActorComponent.K2_DestroyComponent` (`self.BPC_Wings`))
  (`parent.SetBlockHit`))

(fn `UserConstructionScript`
  (`parent.UserConstructionScript`)
  (`/Game/BluePrints/Components/BPC_Wings.InitializeWings` (`self.BPC_Wings`)))