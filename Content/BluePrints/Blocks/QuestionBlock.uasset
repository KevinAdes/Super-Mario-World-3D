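; Question block that Mario can hit once to release an item, such as a Mushroom.
; BeginPlay loops through four static meshes on short delays to fake spinning until the block is hit.
; A MarioBox hit by BP_Mario in a specific state swaps in the used-block mesh and runs SpawnItem.
; SpawnItem selects Mushroom when Mario's PowerState is zero, spawns HitItem above the block, and attempts BlockSpawn through a Mushroom cast.
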(event `self.ReceiveBeginPlay`
  (set `self.Spinning` true)
  (`StaticMeshComponent.SetStaticMesh` (`self.StaticMesh`) "/Game/Models/Blocks/QuestionBlock1.QuestionBlock1" :!label _label)
  (`KismetSystemLibrary.Delay` 0.2)
  (if (`self.Spinning`)
    (`StaticMeshComponent.SetStaticMesh` (`self.StaticMesh`) "/Game/Models/Blocks/QuestionBlock2.QuestionBlock2")
    (`KismetSystemLibrary.Delay` 0.2)
    (if (`self.Spinning`)
      (`StaticMeshComponent.SetStaticMesh` (`self.StaticMesh`) "/Game/Models/Blocks/QuestionBlock3.QuestionBlock3")
      (`KismetSystemLibrary.Delay` 0.2)
      (if (`self.Spinning`)
        (`StaticMeshComponent.SetStaticMesh` (`self.StaticMesh`) "/Game/Models/Blocks/QuestionBlock4.QuestionBlock4")
        (`KismetSystemLibrary.Delay` 0.2)
        (if (`self.Spinning`)
          (goto _label))))))

(event `self.Mario Box.OnComponentHit`
  (params (HitComponent :type "PrimitiveComponent Object Reference") (OtherActor :type "Actor Object Reference") (OtherComp :type "PrimitiveComponent Object Reference") (NormalImpulse :type "Vector Structure") (Hit :type "HitResult Structure (by ref)"))
  (bind _asbp_mario (cast `/Game/BluePrints/BP_Mario` OtherActor))
  (set `self.MarioRef` _asbp_mario)
  (if (`|EnumEquality` (`/Game/BluePrints/BP_Mario.MarioStates` _asbp_mario) "NewEnumerator1")
    (`/Engine/EditorBlueprintResources/StandardMacros.DoOnce` false
      (:`Completed`
        (`self.SetBlockHit`)
        (`self.SpawnItem`)))))

(fn `SetBlockHit`
  (set `self.Spinning` false)
  (set `self.BlockHit` true)
  (`StaticMeshComponent.SetStaticMesh` (`self.StaticMesh`) "/Game/Models/Blocks/HitBlock.HitBlock"))

(fn `SpawnItem`
  (bind _returnvalue (`self.GetTransform`))
  (`|ExecutionSequence`
    (:`then_0`
      (if (== (`/Game/BluePrints/BP_Mario.PowerState` (`self.MarioRef`)) 0)
        (set `self.Hit Item` "/Game/BluePrints/Items/Mushroom.Mushroom_C")))
    (:`then_1`
      (bind _returnvalue_2 (`|SpawnActorFromClass` (`self.Hit Item`) (`KismetMathLibrary.MakeTransform` (`KismetMathLibrary.MakeVector` (.x (.location _returnvalue)) (.y (.location _returnvalue)) (+ (.z (.location _returnvalue)) 40.0)) (.rotation _returnvalue) (.scale _returnvalue)) "AlwaysSpawn" "SelectDefaultAtRuntime" null null))
      (bind _instigator (`Actor.Instigator` _returnvalue_2))
      (`Pawn.SpawnDefaultController` _instigator)
      (bind _asmushroom (cast `/Game/BluePrints/Items/Mushroom` _instigator))
      (`/Game/BluePrints/Items/Mushroom.BlockSpawn` _asmushroom))))

(fn `UserConstructionScript`)