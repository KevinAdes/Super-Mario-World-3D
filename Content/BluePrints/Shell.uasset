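; Shell is a red shell pawn that starts sliding when an actor tagged Mario hits its capsule.
; A Mario hit stores the impact normal as the direction fed to movement input every Tick.
; Other hits while moving reflect that direction off the horizontal hit normal, so the shell ricochets.
; Once moving, an endless Delay loop fakes spinning by cycling four skeletal meshes of different shell views.
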(event `self.ReceiveTick`
  (params (DeltaSeconds :type "Float (single-precision)"))
  (bind _mesh (`self.Mesh`))
  (if (`self.Moving`)
    (`self.AddMovementInput` (`self.Impact Normal`))
    (if (not (`self.Spinning`))
      (set `self.Spinning` true)
      (`SkinnedMeshComponent.SetSkinnedAssetAndUpdate` _mesh "/Game/Models/Koopa/Red/RedShell34.RedShell34" true :!label _label)
      (`KismetSystemLibrary.Delay` 0.2)
      (`SkinnedMeshComponent.SetSkinnedAssetAndUpdate` _mesh "/Game/Models/Koopa/Red/RedShellSide.RedShellSide" true)
      (`KismetSystemLibrary.Delay` 0.2)
      (`SkinnedMeshComponent.SetSkinnedAssetAndUpdate` _mesh "/Game/Models/Koopa/Red/RedShell342.RedShell342" true)
      (`KismetSystemLibrary.Delay` 0.2)
      (`SkinnedMeshComponent.SetSkinnedAssetAndUpdate` _mesh "/Game/Models/Koopa/Red/RedShellFront.RedShellFront" true)
      (`KismetSystemLibrary.Delay` 0.2)
      (goto _label))))

(event `self.CapsuleComponent.OnComponentHit`
  (params (HitComponent :type "PrimitiveComponent Object Reference") (OtherActor :type "Actor Object Reference") (OtherComp :type "PrimitiveComponent Object Reference") (NormalImpulse :type "Vector Structure") (Hit :type "HitResult Structure (by ref)"))
  (bind (_bblockinghit _binitialoverlap _time _distance _location _impactpoint _normal _impactnormal) (`GameplayStatics.BreakHitResult` Hit))
  (if (`self.ActorHasTag` OtherActor "Mario")
    (set `self.Moving` true)
    (set `self.Impact Normal` _impactnormal)
    (elif (`self.Moving`)
      (set `self.Impact Normal` (`KismetMathLibrary.MirrorVectorByNormal` (`self.Impact Normal`) (`KismetMathLibrary.MakeVector` (.x _normal) (.y _normal)))))))

(fn `UserConstructionScript`)