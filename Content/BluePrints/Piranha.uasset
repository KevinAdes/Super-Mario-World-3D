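; Jumping piranha plant enemy that repeatedly leaps out of a pipe, holding off while Mario is near it.
; A timer calls Launch at start and on each ResetVolume overlap; a blocked launch fires when Mario leaves PipeCollider.
; Launch shapes the jump, hover and descent with timed gravity and velocity changes.
; An endless Delay loop animates by swapping skeletal meshes for the mouth and, while spinning, the propeller.
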(event `self.ReceiveBeginPlay`
  (`PrimitiveComponent.IgnoreActorWhenMoving` (`self.Pipe Collider`) (`self.Reset Volume`) true)
  (`PrimitiveComponent.IgnoreActorWhenMoving` (`self.CapsuleComponent`) (`self.Pipe`) true)
  (`KismetSystemLibrary.K2_SetTimerDelegate` (delegate `Launch`) 1.2)
  (`SkinnedMeshComponent.SetSkinnedAssetAndUpdate` (`self.Head`) "/Game/Models/Piranha/RedPiranhaClosed.RedPiranhaClosed" true :!label _label)
  (if (`self.Spinning`)
    (`KismetSystemLibrary.Delay` 0.066667)
    (`SkinnedMeshComponent.SetSkinnedAssetAndUpdate` (`self.Propeller`) "/Game/Models/Piranha/Propeller1.Propeller1" true)
    (`KismetSystemLibrary.Delay` 0.066667)
    (`SkinnedMeshComponent.SetSkinnedAssetAndUpdate` (`self.Propeller`) "/Game/Models/Piranha/Propeller2.Propeller2" true)
    (else
      (`KismetSystemLibrary.Delay` 0.133333)))
  (`SkinnedMeshComponent.SetSkinnedAssetAndUpdate` (`self.Head`) "/Game/Models/Piranha/RedPiranhaOpen.RedPiranhaOpen" true)
  (if (`self.Spinning`)
    (`KismetSystemLibrary.Delay` 0.066667)
    (`SkinnedMeshComponent.SetSkinnedAssetAndUpdate` (`self.Propeller`) "/Game/Models/Piranha/Propeller1.Propeller1" true)
    (`KismetSystemLibrary.Delay` 0.066667)
    (`SkinnedMeshComponent.SetSkinnedAssetAndUpdate` (`self.Propeller`) "/Game/Models/Piranha/Propeller2.Propeller2" true)
    (goto _label)
    (else
      (`KismetSystemLibrary.Delay` 0.133333)
      (goto _label))))

(event `self.CapsuleComponent.OnComponentBeginOverlap`
  (params (OverlappedComponent :type "PrimitiveComponent Object Reference") (OtherActor :type "Actor Object Reference") (OtherComp :type "PrimitiveComponent Object Reference") (OtherBodyIndex :type Integer) (bFromSweep :type Boolean) (SweepResult :type "HitResult Structure (by ref)"))
  (if (== OtherActor (`self.Reset Volume`))
    (`KismetSystemLibrary.K2_SetTimerDelegate` (delegate `Launch`) 1.2)))

(event `Launch`
  (bind _charactermovement (`self.CharacterMovement`))
  (if (`self.Mario Near Pipe`)
    (set `self.Ready for Launch` true)
    (else
      (set `CharacterMovementComponent.GravityScale` 4.179 _charactermovement)
      (set `self.Spinning` false)
      (set `self.Ready for Launch` false)
      (`self.Jump`)
      (`KismetSystemLibrary.Delay` 0.35)
      (set `CharacterMovementComponent.GravityScale` 0.591 _charactermovement)
      (`KismetSystemLibrary.Delay` 0.11)
      (set `self.Spinning` true)
      (`KismetSystemLibrary.Delay` 0.86)
      (set `CharacterMovementComponent.GravityScale` 0.0 _charactermovement)
      (`KismetSystemLibrary.Delay` 0.33)
      (set `CharacterMovementComponent.GravityScale` 0.00536 _charactermovement)
      (`KismetSystemLibrary.Delay` 0.18)
      (set `CharacterMovementComponent.GravityScale` 0.0 _charactermovement)
      (set `MovementComponent.Velocity` (0.0 0.0 -299.0) _charactermovement))))

(event `self.Pipe Collider.OnComponentBeginOverlap`
  (params (OverlappedComponent :type "PrimitiveComponent Object Reference") (OtherActor :type "Actor Object Reference") (OtherComp :type "PrimitiveComponent Object Reference") (OtherBodyIndex :type Integer) (bFromSweep :type Boolean) (SweepResult :type "HitResult Structure (by ref)"))
  (cast `/Game/BluePrints/Mario` OtherActor)
  (set `self.Mario Near Pipe` true))

(event `self.Pipe Collider.OnComponentEndOverlap`
  (params (OverlappedComponent :type "PrimitiveComponent Object Reference") (OtherActor :type "Actor Object Reference") (OtherComp :type "PrimitiveComponent Object Reference") (OtherBodyIndex :type Integer))
  (cast `/Game/BluePrints/Mario` OtherActor)
  (set `self.Mario Near Pipe` false)
  (if (`self.Ready for Launch`)
    (`self.Launch`)))

(fn `UserConstructionScript`)