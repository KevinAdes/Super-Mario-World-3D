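; Mario's pawn on the world map, which moves between linked level points and opens the selected level.
; It starts at the game instance's saved level, falling back to YoshisHouse, and fades in the map HUD.
; Directional input follows neighbor links through LevelMap, moving via a placeholder timeline lerp, then labels the HUD from DT_Levels.
; Clearing the current point blocks input mid-move; selecting saves the level, fades out and loads it.
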(event `self.ReceivePossessed`
  (params (NewController :type "Controller Object Reference")))

(event `self.ReceiveBeginPlay`
  ;[1 1 1] Begin Play
  (`|ExecutionSequence`
    (:`then_0`
      (bind _asbp_game_instance (cast `/Game/BluePrints/GameStuff/BP_GameInstance` (`GameplayStatics.GetGameInstance`)))
      (bind (_value _returnvalue) (`BlueprintMapLibrary.Map_Find` (`self.LevelMap`) (`/Game/BluePrints/GameStuff/BP_GameInstance.CurrentLevel` _asbp_game_instance)))
      (bind _output_get (set `self.CurrentLevelPoint` (select `bool` _returnvalue :`false` (`BlueprintMapLibrary.Map_Find` (`self.LevelMap`) "YoshisHouse") :`true` _value)))
      (`self.K2_SetActorLocation` (`SceneComponent.K2_GetComponentLocation` (`/Game/BluePrints/Map/BP_LevelPoint.DefaultSceneRoot` _output_get))))
    (:`then_1`
      (bind _asbp_map_hud (cast `/Game/GameModeDefaults/BP_MapHud` (`PlayerController.GetHUD` (`GameplayStatics.GetPlayerController` 0))))
      (bind _output_get_2 (set `self.MapHud` (`/Game/GameModeDefaults/BP_MapHud.WBP_MapHud` _asbp_map_hud)))
      (`/Game/BluePrints/Widgets/HUD/WBP_MapHud.FadeIn` _output_get_2))))

(event `InputAction|MapUp`
  (params (Key :type "Key Structure"))
  ;[1 1 1] HandleUpInput
  (:`Pressed`
    (bind _uplevel (`/Game/BluePrints/Map/BP_LevelPoint.UpLevel` (`self.CurrentLevelPoint`))
      (:`then`
        (bind (_value _returnvalue) (`BlueprintMapLibrary.Map_Find` (`self.LevelMap`) (`/Game/BluePrints/Map/BP_LevelPoint.LevelName` _uplevel)))
        (if _returnvalue
          (`self.MoveTo` _value)
          (set `self.CurrentLevelPoint` null)))
      (:`else`))))

(event `UpdateLevel`)

(event `InputAction|MapLeft`
  (params (Key :type "Key Structure"))
  ;[1 1 1] Handle Left Input
  (:`Pressed`
    (bind _leftlevel (`/Game/BluePrints/Map/BP_LevelPoint.LeftLevel` (`self.CurrentLevelPoint`))
      (:`then`
        (bind (_value _returnvalue) (`BlueprintMapLibrary.Map_Find` (`self.LevelMap`) (`/Game/BluePrints/Map/BP_LevelPoint.LevelName` _leftlevel)))
        (if _returnvalue
          (`self.MoveTo` _value)
          (set `self.CurrentLevelPoint` null)))
      (:`else`))))

(event `MoveTo`
  (params (TargetLevel :type "/Game/BluePrints/Map/BP_LevelPoint Object Reference"))
  (bind _levelname (`/Game/BluePrints/Map/BP_LevelPoint.LevelName` TargetLevel))
  ;[1 1 1] Linearly interpolate mario from level point to level point. MUST be replaced with a more robust system eventually
  (bind (_direction _lerpalpha) (`Timeline|MoveTimeline` :!via `PlayFromStart`)
    (:`Update`
      (`self.K2_SetActorLocation` (`KismetMathLibrary.VLerp` (`self.K2_GetActorLocation`) (`SceneComponent.K2_GetComponentLocation` (`/Game/BluePrints/Map/BP_LevelPoint.DefaultSceneRoot` TargetLevel)) _lerpalpha)))
    (:`Finished`
      (set `self.CurrentLevelPoint` TargetLevel)
      (bind _returnvalue (`|GetDataTableRow` "/Game/Data/DT_Levels.DT_Levels" _levelname)
        (:`then`
          (`/Game/BluePrints/Widgets/HUD/WBP_MapHud.SetLevelLabel` (`self.MapHud`) (`KismetTextLibrary.Conv_StringToText` (`.DisplayName` (break `LevelData` _returnvalue)))))
        (:`RowNotFound`
          (`KismetSystemLibrary.PrintText` (`|FormatText` "Row Not Found {RowName}" (`KismetTextLibrary.Conv_NameToText` _levelname))))))))

(event `InputAction|MapRight`
  (params (Key :type "Key Structure"))
  ;[1 1 1] HandleRightInput
  (:`Pressed`
    (bind _rightlevel (`/Game/BluePrints/Map/BP_LevelPoint.RightLevel` (`self.CurrentLevelPoint`))
      (:`then`
        (bind (_value _returnvalue) (`BlueprintMapLibrary.Map_Find` (`self.LevelMap`) (`/Game/BluePrints/Map/BP_LevelPoint.LevelName` _rightlevel)))
        (if _returnvalue
          (`self.MoveTo` _value)
          (set `self.CurrentLevelPoint` null)))
      (:`else`))))

(event `InputAction|MapSelect`
  (params (Key :type "Key Structure"))
  ;[1 1 1] If there is a valid Current level, select it
  (:`Pressed`
    (bind _currentlevelpoint (`self.CurrentLevelPoint`)
      (:`then`
        (bind _asbp_game_instance (cast `/Game/BluePrints/GameStuff/BP_GameInstance` (`GameplayStatics.GetGameInstance`)))
        (set `/Game/BluePrints/GameStuff/BP_GameInstance.CurrentLevel` (`/Game/BluePrints/Map/BP_LevelPoint.LevelName` _currentlevelpoint) _asbp_game_instance)
        (`/Game/BluePrints/Widgets/HUD/WBP_MapHud.FadeOut` (`self.MapHud`))
        (`KismetSystemLibrary.Delay` 1.0)
        (`GameplayStatics.OpenLevelBySoftObjectPtr` (`/Game/BluePrints/Map/BP_LevelPoint.LevelReference` _currentlevelpoint)))
      (:`else`))))

(event `InputAction|MapDown`
  (params (Key :type "Key Structure"))
  ;[1 1 1] HandleDownInput
  (:`Pressed`
    (bind _downlevel (`/Game/BluePrints/Map/BP_LevelPoint.DownLevel` (`self.CurrentLevelPoint`))
      (:`then`
        (bind (_value _returnvalue) (`BlueprintMapLibrary.Map_Find` (`self.LevelMap`) (`/Game/BluePrints/Map/BP_LevelPoint.LevelName` _downlevel)))
        (if _returnvalue
          (`self.MoveTo` _value)
          (set `self.CurrentLevelPoint` null)))
      (:`else`))))

(fn `SetPositionByLevel`)

(fn `UserConstructionScript`)