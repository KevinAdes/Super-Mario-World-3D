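; BP_LevelPoint is a level node on the map that represents a playable level and can open it.
; On BeginPlay, an unlocked point registers itself in the LevelMap of the BP_MapMario player pawn, keyed by LevelName.
; Its OpenLevel function loads the assigned LevelReference by object reference.
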(event `self.ReceiveBeginPlay`
  (if (`self.Unlocked`)
    (bind _asbp_map_mario (cast `/Game/BluePrints/Map/BP_MapMario` (`GameplayStatics.GetPlayerPawn` 0)))
    (`BlueprintMapLibrary.Map_Add` (`/Game/BluePrints/Map/BP_MapMario.LevelMap` _asbp_map_mario) (`self.LevelName`) self)))

(fn `OpenLevel`
  (`GameplayStatics.OpenLevelBySoftObjectPtr` (`self.LevelReference`)))

(fn `UserConstructionScript`)