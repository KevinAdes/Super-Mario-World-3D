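; BPC_Wings is a component that gives its owning actor a pair of animated flapping wings.
; InitializeWings, not called within this Blueprint, adds two static mesh components to the owner, positions them by per-side location and yaw, and mirrors the right with negative X scale.
; FlapWings toggles both between open and closed meshes as a simple mesh-swap animation.
; BeginPlay starts a looping timer, presumably driving the flap, though its bound function is not shown.
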(event `self.ReceiveBeginPlay`
  (`KismetSystemLibrary.K2_SetTimerDelegate` (`|CreateDelegate` :!event `FlapWings`) 0.4 true))

(fn `FlapWings`
  (bind _output_get (set `self.Closed` (not (stale _output_get))))
  (bind _returnvalue (select `bool` _output_get :`false` "/Game/Models/Wings/Wings_Closed.Wings_Closed" :`true` "/Game/Models/Wings/Wings_Open.Wings_Open" :!type "StaticMesh Object Reference"))
  (`StaticMeshComponent.SetStaticMesh` (`self.RightWing`) _returnvalue)
  (`StaticMeshComponent.SetStaticMesh` (`self.LeftWing`) _returnvalue))

(fn `InitializeWings`
  (bind _returnvalue (`self.GetOwner`))
  (`|ExecutionSequence`
    (:`then_1`
      (bind _returnvalue_2 (`|AddComponentByClass` :`self` _returnvalue :`Class` "/Script/Engine.StaticMeshComponent"))
      (set `self.RightWing` _returnvalue_2)
      (bind _returnvalue_3 (`|AddComponentByClass` :`self` _returnvalue :`Class` "/Script/Engine.StaticMeshComponent"))
      (set `self.LeftWing` _returnvalue_3))
    (:`then_2`
      (`StaticMeshComponent.SetStaticMesh` (`self.RightWing`) "/Game/Models/Wings/Wings_Open.Wings_Open")
      (`StaticMeshComponent.SetStaticMesh` (`self.LeftWing`) "/Game/Models/Wings/Wings_Open.Wings_Open")
      (`self.K2_AddLocalTransform` (`self.RightWing`) (`KismetMathLibrary.MakeTransform` (`self.RightWingLocation`) (`KismetMathLibrary.MakeRotator` 0.0 0.0 (`self.RightWingRotation`)) (-1.0 1.0 1.0)) false false)
      (`self.K2_AddLocalTransform` (`self.LeftWing`) (`KismetMathLibrary.MakeTransform` (`self.LeftWingLocation`) (`KismetMathLibrary.MakeRotator` 0.0 0.0 (`self.LeftWingRotation`))) false false))
    (:`then_3`
      (bind _output_get (set `self.Closed` (not (stale _output_get))))
      (bind _returnvalue_4 (select `bool` _output_get :`false` "/Game/Models/Wings/Wings_Closed.Wings_Closed" :`true` "/Game/Models/Wings/Wings_Open.Wings_Open" :!type "StaticMesh Object Reference"))
      (`StaticMeshComponent.SetStaticMesh` (`self.RightWing`) _returnvalue_4)
      (`StaticMeshComponent.SetStaticMesh` (`self.LeftWing`) _returnvalue_4))))