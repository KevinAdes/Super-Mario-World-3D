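; Jumping Piranha Plant enemy that leaps from a pipe, kills Mario on capsule contact, and bounces him if he spin-jumps onto its StompBox.
; Launch scripts the rise, hover and descent with timed velocity and gravity changes, re-arming on a timer when it overlaps ResetVolume.
; PipeCollider holds back a due launch while Mario is near.
; A looping mesh swap animates the mouth, plus the propeller while spinning.
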(event `self.ReceiveBeginPlay`
  (`PrimitiveComponent.IgnoreActorWhenMoving` (`self.Pipe Collider`) (`self.Reset Volume`) true)
  (`PrimitiveComponent.IgnoreActorWhenMoving` (`self.CapsuleComponent`) (`self.Pipe`) true)
  (`KismetSystemLibrary.K2_SetTimerDelegate` (delegate `Launch`) 1.2)
  (`SkinnedMeshComponent.SetSkinnedAssetAndUpdate` (`self.Head`) "/Game/Models/Piranha/RedPiranhaClosed.RedPiranhaClosed" true :!label _label)
  (if (`self.Spinning`)
    (`KismetSystemLibrary.Delay` 0.066667)
    (`SkinnedMeshComponent.SetSkinnedAssetAndUpdate` (`self.Propeller`) "/Game/Models/Piranha/Propeller1.Propeller1" true)
    (`KismetSystemLibrary.Delay` 0.066667)
    (`SkinnedMeshComponent.SetSkinnedAssetAndUpdate` (`self.Propeller`) "/Game/Models/Piranha/Propeller2.Propeller2" true)
    (else
      (`KismetSystemLibrary.Delay` 0.133333)))
  (`SkinnedMeshComponent.SetSkinnedAssetAndUpdate` (`self.Head`) "/Game/Models/Piranha/RedPiranhaOpen.RedPiranhaOpen" true)
  (if (`self.Spinning`)
    (`KismetSystemLibrary.Delay` 0.066667)
    (`SkinnedMeshComponent.SetSkinnedAssetAndUpdate` (`self.Propeller`) "/Game/Models/Piranha/Propeller1.Propeller1" true)
    (`KismetSystemLibrary.Delay` 0.066667)
    (`SkinnedMeshComponent.SetSkinnedAssetAndUpdate` (`self.Propeller`) "/Game/Models/Piranha/Propeller2.Propeller2" true)
    (goto _label)
    (else
      (`KismetSystemLibrary.Delay` 0.133333)
      (goto _label))))

(event `self.CapsuleComponent.OnComponentBeginOverlap`
  (params (OverlappedComponent :type "PrimitiveComponent Object Reference") (OtherActor :type "Actor Object Reference") (OtherComp :type "PrimitiveComponent Object Reference") (OtherBodyIndex :type Integer) (bFromSweep :type Boolean) (SweepResult :type "HitResult Structure (by ref)"))
  (if (== OtherActor (`self.Reset Volume`))
    (`KismetSystemLibrary.K2_SetTimerDelegate` (delegate `Launch`) 1.2)
    (else
      (bind _asmario (cast `/Game/BluePrints/BP_Mario` OtherActor))
      (`/Engine/EditorBlueprintResources/StandardMacros.DoOnce` false
        (:`Completed`
          (`/Game/BluePrints/BP_Mario.Kill` _asmario))))))

(event `Launch`
  (bind _charactermovement (`self.CharacterMovement`))
  (if (`self.Mario Near Pipe`)
    (set `self.Ready for Launch` true)
    (else
      (set `MovementComponent.Velocity` (0.0 0.0 0.0) _charactermovement)
      (set `CharacterMovementComponent.GravityScale` 4.179 _charactermovement)
      (set `self.Spinning` false)
      (set `self.Ready for Launch` false)
      (`self.Jump`)
      (`KismetSystemLibrary.Delay` 0.35)
      (set `CharacterMovementComponent.GravityScale` 0.591 _charactermovement)
      (set `MovementComponent.Velocity` (0.0 0.0 647.0) _charactermovement)
      (`KismetSystemLibrary.Delay` 0.11)
      (set `self.Spinning` true)
      (`KismetSystemLibrary.Delay` 0.86)
      (set `CharacterMovementComponent.GravityScale` 0.0 _charactermovement)
      (set `MovementComponent.Velocity` (0.0 0.0 0.0) _charactermovement)
      (`KismetSystemLibrary.Delay` 0.33)
      (set `CharacterMovementComponent.GravityScale` 0.00536 _charactermovement)
      (`KismetSystemLibrary.Delay` 0.18)
      (set `CharacterMovementComponent.GravityScale` 0.0 _charactermovement)
      (set `MovementComponent.Velocity` (0.0 0.0 -299.0) _charactermovement))))

(event `self.Pipe Collider.OnComponentBeginOverlap`
  (params (OverlappedComponent :type "PrimitiveComponent Object Reference") (OtherActor :type "Actor Object Reference") (OtherComp :type "PrimitiveComponent Object Reference") (OtherBodyIndex :type Integer) (bFromSweep :type Boolean) (SweepResult :type "HitResult Structure (by ref)"))
  (cast `/Game/BluePrints/BP_Mario` OtherActor)
  (set `self.Mario Near Pipe` true))

(event `self.Pipe Collider.OnComponentEndOverlap`
  (params (OverlappedComponent :type "PrimitiveComponent Object Reference") (OtherActor :type "Actor Object Reference") (OtherComp :type "PrimitiveComponent Object Reference") (OtherBodyIndex :type Integer))
  (cast `/Game/BluePrints/BP_Mario` OtherActor)
  (set `self.Mario Near Pipe` false)
  (if (`self.Ready for Launch`)
    (`self.Launch`)))

(event `self.StompBox.OnComponentBeginOverlap`
  (params (OverlappedComponent :type "PrimitiveComponent Object Reference") (OtherActor :type "Actor Object Reference") (OtherComp :type "PrimitiveComponent Object Reference") (OtherBodyIndex :type Integer) (bFromSweep :type Boolean) (SweepResult :type "HitResult Structure (by ref)"))
  (bind _asmario (cast `/Game/BluePrints/BP_Mario` OtherActor))
  (if (`/Game/BluePrints/BP_Mario.SpinJumping` _asmario)
    (`/Engine/EditorBlueprintResources/StandardMacros.DoOnce` false :!label _label_2
      (:`Completed`
        (bind _charactermovement (`Character.CharacterMovement` _asmario))
        (set `CharacterMovementComponent.JumpZVelocity` 0.0 _charactermovement)
        (set `MovementComponent.Velocity` (0.0 0.0 0.0) _charactermovement)
        (if (`/Game/BluePrints/BP_Mario.JumpHeld` _asmario)
          (set `CharacterMovementComponent.GravityScale` 6.93 _charactermovement)
          (`CharacterMovementComponent.AddImpulse` _charactermovement (0.0 0.0 3000.0) true)
          (else
            (set `CharacterMovementComponent.GravityScale` 16.3 _charactermovement)
            (`CharacterMovementComponent.AddImpulse` _charactermovement (0.0 0.0 2910.0) true)))
        (`KismetSystemLibrary.DelayUntilNextTick`)
        (goto _label_2 :!via `Reset`)))))

(fn `UserConstructionScript`)