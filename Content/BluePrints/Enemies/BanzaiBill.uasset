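; Banzai Bill enemy pawn that homes in on BP_Mario and can kill him or be stomped.
; It aims at Mario on BeginPlay, retargets whenever PawnSensing sees him, and eases its horizontal heading toward that vector each Tick while moving forward.
; Body overlaps share a DoOnce that kills Mario.
; StompBox overlaps pass a Shoebox check, then bounce Mario, disable collision on the SpawnActor reference and destroy the Bill.
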(event `self.ReceiveBeginPlay`
  (bind _returnvalue (`GameplayStatics.GetActorOfClass` "/Game/BluePrints/BP_Mario.BP_Mario_C"))
  (bind (_returnvalue_x _returnvalue_y) (`KismetMathLibrary.BreakVector` (- (`self.K2_GetActorLocation` _returnvalue) (`self.K2_GetActorLocation` self))))
  (bind _output_get (set `self.Move Vector` (`KismetMathLibrary.MakeVector` _returnvalue_x _returnvalue_y)))
  (set `self.Vector to lerp to` _output_get)
  (`self.SetActorTickEnabled` true))

(event `self.PawnSensing.OnSeePawn`
  (params (Pawn :type "Pawn Object Reference"))
  (bind _asbp_mario (cast `/Game/BluePrints/BP_Mario` Pawn))
  (bind (_returnvalue_x _returnvalue_y) (`KismetMathLibrary.BreakVector` (- (`self.K2_GetActorLocation` _asbp_mario) (`self.K2_GetActorLocation` self))))
  (set `self.Vector to lerp to` (`KismetMathLibrary.MakeVector` _returnvalue_x _returnvalue_y)))

(event `self.ReceiveTick`
  (params (DeltaSeconds :type "Float (single-precision)"))
  (bind _returnvalue (`KismetMathLibrary.VLerp` (`self.Move Vector`) (`self.Vector to lerp to`) 0.5))
  (`self.K2_SetActorRotation` (`KismetMathLibrary.Conv_VectorToRotator` _returnvalue))
  (`self.AddMovementInput` _returnvalue 1.0 true)
  (set `self.Move Vector` _returnvalue))

(event `self.Capsule.OnComponentBeginOverlap`
  (params (OverlappedComponent :type "PrimitiveComponent Object Reference") (OtherActor :type "Actor Object Reference") (OtherComp :type "PrimitiveComponent Object Reference") (OtherBodyIndex :type Integer) (bFromSweep :type Boolean) (SweepResult :type "HitResult Structure (by ref)"))
  (bind _asbp_mario (cast `/Game/BluePrints/BP_Mario` OtherActor))
  (`/Engine/EditorBlueprintResources/StandardMacros.DoOnce` false :!label _label
    (:`Completed`
      (`/Game/BluePrints/BP_Mario.Kill` _asbp_mario)
      (`/Game/BluePrints/BP_Mario.Kill` (stale `self.Cylinder.OnComponentBeginOverlap` _asbp_mario))
      (`/Game/BluePrints/BP_Mario.Kill` (stale `self.Capsule1.OnComponentBeginOverlap` _asbp_mario)))))

(event `self.Cylinder.OnComponentBeginOverlap`
  (params (OverlappedComponent :type "PrimitiveComponent Object Reference") (OtherActor :type "Actor Object Reference") (OtherComp :type "PrimitiveComponent Object Reference") (OtherBodyIndex :type Integer) (bFromSweep :type Boolean) (SweepResult :type "HitResult Structure (by ref)"))
  (bind _asbp_mario (cast `/Game/BluePrints/BP_Mario` OtherActor))
  (goto _label))

(event `self.Capsule1.OnComponentBeginOverlap`
  (params (OverlappedComponent :type "PrimitiveComponent Object Reference") (OtherActor :type "Actor Object Reference") (OtherComp :type "PrimitiveComponent Object Reference") (OtherBodyIndex :type Integer) (bFromSweep :type Boolean) (SweepResult :type "HitResult Structure (by ref)"))
  (bind _asbp_mario (cast `/Game/BluePrints/BP_Mario` OtherActor))
  (goto _label))

(event `self.StompBox.OnComponentBeginOverlap`
  (params (OverlappedComponent :type "PrimitiveComponent Object Reference") (OtherActor :type "Actor Object Reference") (OtherComp :type "PrimitiveComponent Object Reference") (OtherBodyIndex :type Integer) (bFromSweep :type Boolean) (SweepResult :type "HitResult Structure (by ref)"))
  (`self.JumpCheck` OtherActor OtherComp)
  (`/Game/BluePrints/BP_Mario.EnemyBounce` (`self.As Mario`) :!label _label_2)
  (`PrimitiveComponent.SetCollisionEnabled` (`TriggerBase.CollisionComponent` (`self.SpawnActor`)) "NoCollision")
  (`self.K2_DestroyActor`))

(event `self.StompBox1.OnComponentBeginOverlap`
  (params (OverlappedComponent :type "PrimitiveComponent Object Reference") (OtherActor :type "Actor Object Reference") (OtherComp :type "PrimitiveComponent Object Reference") (OtherBodyIndex :type Integer) (bFromSweep :type Boolean) (SweepResult :type "HitResult Structure (by ref)"))
  (`self.JumpCheck` OtherActor OtherComp)
  (goto _label_2))

(fn `UserConstructionScript`)