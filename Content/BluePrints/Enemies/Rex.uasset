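; Rex enemy that kills Mario on contact, takes two stomps to defeat, and dies instantly to spin jumps or non-idle shells.
; It follows an optional Path actor or walks freely, line-tracing for ledges to turn, and reverses or deflects off walls, enemies and idle shells.
; Walking animates by swapping skeletal meshes on a delay loop.
; The first stomp shrinks its collision, switches mesh set and resets speed, while each stomp bounces Mario.
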(event `self.ReceiveBeginPlay`
  (bind _damaged (`self.Damaged`))
  (bind _stepduration (`self.StepDuration`))
  (bind _stepduration_2 (`self.StepDuration`))
  (bind _damaged_2 (`self.Damaged`))
  (`self.Set Path Speed` (`CharacterMovementComponent.MaxWalkSpeed` (`self.CharacterMovement`))
    (:`Is Not Valid`
      (set `self.Movement Vector` (`SceneComponent.GetForwardVector` (`self.Mesh`))))
    (:`then`
      (`PrimitiveComponent.IgnoreActorWhenMoving` (`self.CapsuleComponent`) (`self.Path`) false)))
  (`SkinnedMeshComponent.SetSkinnedAssetAndUpdate` (`self.Mesh`) (`|GetArrayItem` (`self.Meshes`) (`self.Still`)) true :!label _label)
  (`KismetSystemLibrary.Delay` _stepduration)
  (if (not _damaged_2)
    (`SkinnedMeshComponent.SetSkinnedAssetAndUpdate` (`self.Mesh`) (`|GetArrayItem` (`self.Meshes`) (`self.Step 1`)) true)
    (`KismetSystemLibrary.Delay` _stepduration)
    (if (not _damaged_2)
      (`SkinnedMeshComponent.SetSkinnedAssetAndUpdate` (`self.Mesh`) (`|GetArrayItem` (`self.Meshes`) (`self.Still`)) true)
      (`KismetSystemLibrary.Delay` _stepduration_2)
      (if (not _damaged)
        (`SkinnedMeshComponent.SetSkinnedAssetAndUpdate` (`self.Mesh`) (`|GetArrayItem` (`self.Meshes`) (`self.Step 2`)) true)
        (`KismetSystemLibrary.Delay` _stepduration_2)
        (if (not _damaged)
          (goto _label))))))

(event `self.ReceiveTick`
  (params (DeltaSeconds :type "Float (single-precision)"))
  (bind (_returnvalue_x _returnvalue_y _returnvalue_z) (`KismetMathLibrary.BreakVector` (`self.K2_GetActorLocation`)))
  (bind _movement_vector (`self.Movement Vector`))
  (bind _mesh (`self.Mesh`))
  (bind _mesh_2 (`self.Mesh`))
  (bind _charactermovement (`self.CharacterMovement`))
  (bind (_returnvalue_x_2 _returnvalue_y_2 _returnvalue_z_2) (`KismetMathLibrary.BreakVector` (`CharacterMovementComponent.GetLastUpdateVelocity` _charactermovement)))
  (bind _returnvalue (`SceneComponent.K2_GetComponentRotation` _mesh))
  (bind _returnvalue_2 (`SceneComponent.K2_GetComponentLocation` _mesh_2))
  (bind _returnvalue_3 (`SceneComponent.K2_GetComponentLocation` _mesh))
  (bind _returnvalue_4 (`SceneComponent.K2_GetComponentRotation` _mesh_2))
  (bind _returnvalue_5 (`SceneComponent.K2_GetComponentToWorld` (`/Game/BluePrints/LevelStuff/Path.Reference point` (`self.Path`))))
  (bind (_returnvalue_x_3 _returnvalue_y_3) (`KismetMathLibrary.BreakVector` (* (`KismetMathLibrary.Normal` _movement_vector) (`CharacterMovementComponent.MaxWalkSpeed` _charactermovement))))
  (bind _returnvalue_6 (+ (`KismetMathLibrary.GetForwardVector` _returnvalue_4) (`KismetMathLibrary.GetRightVector` _returnvalue_4)))
  (`/Engine/EditorBlueprintResources/StandardMacros.IsValid` (`self.Path`)
    (:`Is Valid`
      (`self.K2_SetActorTransform` (`KismetMathLibrary.MakeTransform` (`KismetMathLibrary.MakeVector` (.x (.location _returnvalue_5)) (.y (.location _returnvalue_5)) _returnvalue_z) (.rotation _returnvalue_5)) true))
    (:`Is Not Valid`
      (bind (_outhit _returnvalue_7) (`KismetSystemLibrary.LineTraceSingleForObjects` _returnvalue_3 (+ _returnvalue_3 (* (+ (`KismetMathLibrary.GetForwardVector` _returnvalue) (* (`KismetMathLibrary.GetUpVector` _returnvalue) (0.0 0.0 -1.0))) (400.0 400.0 400.0))) (`self.NewVar_0`) true))
      (if (not _returnvalue_7)
        (set `self.Movement Vector` _returnvalue_6)
        (`self.K2_SetActorRotation` (`KismetMathLibrary.Conv_VectorToRotator` _returnvalue_6)))
      (set `MovementComponent.Velocity` (`KismetMathLibrary.MakeVector` _returnvalue_x_3 _returnvalue_y_3 _returnvalue_z_2) _charactermovement)
      (`self.K2_SetActorRotation` (`KismetMathLibrary.FindLookAtRotation` _returnvalue_2 (+ _returnvalue_2 _movement_vector))))))

(event `self.CapsuleComponent.OnComponentBeginOverlap`
  (params (OverlappedComponent :type "PrimitiveComponent Object Reference") (OtherActor :type "Actor Object Reference") (OtherComp :type "PrimitiveComponent Object Reference") (OtherBodyIndex :type Integer) (bFromSweep :type Boolean) (SweepResult :type "HitResult Structure (by ref)"))
  (bind _asmario (cast `/Game/BluePrints/Mario` OtherActor))
  (if (> (`self.Health`) 0)
    (`/Game/BluePrints/Mario.Kill` _asmario)))

(event `self.StompBox.OnComponentBeginOverlap`
  (params (OverlappedComponent :type "PrimitiveComponent Object Reference") (OtherActor :type "Actor Object Reference") (OtherComp :type "PrimitiveComponent Object Reference") (OtherBodyIndex :type Integer) (bFromSweep :type Boolean) (SweepResult :type "HitResult Structure (by ref)"))
  (bind _mesh (`self.Mesh`))
  (bind _capsulecomponent (`self.CapsuleComponent`))
  (bind _stompbox (`self.StompBox`))
  (bind _as_mario (`self.As Mario`))
  (bind _as_mario_2 (`self.As Mario`))
  (bind _as_mario_3 (`self.As Mario`))
  (bind _health (`self.Health`))
  (bind _charactermovement (`Character.CharacterMovement` _as_mario))
  (bind _charactermovement_2 (`Character.CharacterMovement` _as_mario_2))
  (bind _charactermovement_3 (`Character.CharacterMovement` _as_mario_3))
  (bind _asmario (cast `/Game/BluePrints/Mario` OtherActor))
  (bind _output_get (set `self.As Mario` _asmario))
  (`self.StopJumping` _output_get)
  (if (`/Game/BluePrints/Mario.SpinJumping` _output_get)
    (`/Engine/EditorBlueprintResources/StandardMacros.DoOnce` false
      (:`Completed`
        (set `CharacterMovementComponent.JumpZVelocity` 0.0 _charactermovement_2)
        (set `MovementComponent.Velocity` (0.0 0.0 0.0) _charactermovement_2)
        (if (`/Game/BluePrints/Mario.JumpHeld` _as_mario_2)
          (set `CharacterMovementComponent.GravityScale` 6.93 _charactermovement_2)
          (`CharacterMovementComponent.AddImpulse` _charactermovement_2 (0.0 0.0 3000.0) true)
          (else
            (set `CharacterMovementComponent.GravityScale` 16.3 _charactermovement_2)
            (`CharacterMovementComponent.AddImpulse` _charactermovement_2 (0.0 0.0 2910.0) true)))
        (`self.K2_DestroyActor`)))
    (elif (and (== (`/Game/BluePrints/Mario.Shoebox` _asmario) OtherComp) (not (`self.Damaged`)))
      (`/Engine/EditorBlueprintResources/StandardMacros.DecrementInt` _health
        (:`  `
          (set `self.Damaged` true)
          (bind _output_get_2 (set `CharacterMovementComponent.MaxWalkSpeed` 0.0 (`self.CharacterMovement`)))
          (`self.Set Path Speed` _output_get_2
            (:`Is Not Valid`
              _)
            (:`then`
              _))
          (if (== _health 1)
            (`SkinnedMeshComponent.SetSkinnedAssetAndUpdate` _mesh "/Game/Models/Rex/RexMidSquish.RexMidSquish" true)
            (`CapsuleComponent.SetCapsuleSize` _capsulecomponent 88.0 103.0 true)
            (`SceneComponent.K2_SetRelativeLocation` _stompbox (14.0 0.0 103.0) false false)
            (`/Engine/EditorBlueprintResources/StandardMacros.DoOnce` false
              (:`Completed`
                (set `CharacterMovementComponent.JumpZVelocity` 0.0 _charactermovement)
                (set `MovementComponent.Velocity` (0.0 0.0 0.0) _charactermovement)
                (if (`/Game/BluePrints/Mario.JumpHeld` _as_mario)
                  (set `CharacterMovementComponent.GravityScale` 6.93 _charactermovement)
                  (`CharacterMovementComponent.AddImpulse` _charactermovement (0.0 0.0 3000.0) true)
                  (else
                    (set `CharacterMovementComponent.GravityScale` 16.3 _charactermovement)
                    (`CharacterMovementComponent.AddImpulse` _charactermovement (0.0 0.0 2910.0) true)))
                (set `self.Step 1` 5)
                (set `self.Step 2` 6)
                (set `self.Still` 4)
                (`KismetSystemLibrary.Delay` 0.15)
                (set `self.Damaged` false)
                (bind _output_get_3 (set `CharacterMovementComponent.MaxWalkSpeed` 698.0 (`self.CharacterMovement`)))
                (`self.Set Path Speed` _output_get_3
                  (:`Is Not Valid`
                    _)
                  (:`then`
                    _))
                (`CapsuleComponent.SetCapsuleSize` (`self.CapsuleComponent`) 69.0 74.0 true)
                (`SceneComponent.K2_SetRelativeLocation` (`self.StompBox`) (3.0 0.0 52.0) false false)
                (goto _label)))
            (else
              (`SkinnedMeshComponent.SetSkinnedAssetAndUpdate` _mesh "/Game/Models/Rex/RexFullSquish.RexFullSquish" true)
              (`CapsuleComponent.SetCapsuleSize` _capsulecomponent 30.0 30.0 true)
              (`PrimitiveComponent.SetCollisionEnabled` _stompbox "NoCollision")
              (`/Engine/EditorBlueprintResources/StandardMacros.DoOnce` false
                (:`Completed`
                  (set `CharacterMovementComponent.JumpZVelocity` 0.0 _charactermovement_3)
                  (set `MovementComponent.Velocity` (0.0 0.0 0.0) _charactermovement_3)
                  (if (`/Game/BluePrints/Mario.JumpHeld` _as_mario_3)
                    (set `CharacterMovementComponent.GravityScale` 6.93 _charactermovement_3)
                    (`CharacterMovementComponent.AddImpulse` _charactermovement_3 (0.0 0.0 3000.0) true)
                    (else
                      (set `CharacterMovementComponent.GravityScale` 16.3 _charactermovement_3)
                      (`CharacterMovementComponent.AddImpulse` _charactermovement_3 (0.0 0.0 2910.0) true)))
                  (`KismetSystemLibrary.Delay` 1.0)
                  (`self.K2_DestroyActor`))))))))))

(event `self.CapsuleComponent.OnComponentHit`
  (params (HitComponent :type "PrimitiveComponent Object Reference") (OtherActor :type "Actor Object Reference") (OtherComp :type "PrimitiveComponent Object Reference") (NormalImpulse :type "Vector Structure") (Hit :type "HitResult Structure (by ref)"))
  (bind (_bblockinghit _binitialoverlap _time _distance _location _impactpoint _normal) (`GameplayStatics.BreakHitResult` Hit))
  (bind _returnvalue (`self.K2_GetActorLocation`))
  (bind _path (`self.Path`))
  (cast `/Game/BluePrints/Mario` OtherActor
    (:`CastFailed`
      (bind _asshell (cast `/Game/BluePrints/Items/Shell` OtherActor)
        (:`then`
          (switch `/Game/BluePrints/Enums/EHoldStates` (`/Game/BluePrints/Items/Shell.States` _asshell)
            (:`NewEnumerator0`
              (`/Engine/EditorBlueprintResources/StandardMacros.IsValid` _path :!label _label_2
                (:`Is Valid`
                  (`/Engine/EditorBlueprintResources/StandardMacros.DoOnce` false :!label _label_3
                    (:`Completed`
                      (set `/Game/BluePrints/LevelStuff/Path.FlipDir` (not (`/Game/BluePrints/LevelStuff/Path.FlipDir` _path)) _path)
                      (`KismetSystemLibrary.Delay` 0.2)
                      (goto _label_3 :!via `Reset`))))
                (:`Is Not Valid`
                  (bind _output_get (set `self.Movement Vector` (`KismetMathLibrary.MirrorVectorByNormal` (`self.Movement Vector`) (`KismetMathLibrary.MakeVector` (.x _normal) (.y _normal)))))
                  (`self.K2_SetActorRotation` (`KismetMathLibrary.FindLookAtRotation` _returnvalue (+ _returnvalue _output_get))))))
            (:`NewEnumerator1`
              (`self.K2_DestroyActor` :!label _label_4))
            (:`NewEnumerator3`
              (`self.K2_DestroyActor` _asshell)
              (goto _label_4))
            (:`NewEnumerator2`
              (goto _label_4))
            (:`NewEnumerator4`
              (goto _label_4))))
        (:`CastFailed`
          (if (or (`self.ActorHasTag` OtherActor "Wall") (`self.ActorHasTag` OtherActor "Enemy"))
            (goto _label_2)))))))

(fn `UserConstructionScript`)