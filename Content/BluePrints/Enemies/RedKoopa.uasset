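; Red Koopa enemy character that walks forward along its mesh's facing, or starts out in a slide.
; Walking is animated flipbook-style by swapping skeletal meshes between step and still poses on a delay loop that stops once Damaged is set.
; A starting slide uses the sixth mesh and the KoopaMovementComponent's slide; switching from custom movement to walking swaps the mesh, waits briefly, clears Slide and restarts the walk loop.
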(event `self.K2_OnMovementModeChanged`
  (params (PrevMovementMode :type "EMovementMode Enum" :default "MOVE_None") (NewMovementMode :type "EMovementMode Enum" :default "MOVE_None") (PrevCustomMode :type Byte) (NewCustomMode :type Byte))
  (bind _damaged (`self.Damaged`))
  (bind _stepduration (`self.StepDuration`))
  (bind _stepduration_2 (`self.StepDuration`))
  (bind _damaged_2 (`self.Damaged`))
  (if (and (`|EnumEquality` PrevMovementMode "MOVE_Custom") (`|EnumEquality` NewMovementMode "MOVE_Walking"))
    (`SkinnedMeshComponent.SetSkinnedAssetAndUpdate` (`self.Mesh`) (`|GetArrayItem` (`self.Meshes`)) false)
    (`KismetSystemLibrary.Delay` 1.0)
    (set `self.Slide` false)
    (`SkinnedMeshComponent.SetSkinnedAssetAndUpdate` (`self.Mesh`) (`|GetArrayItem` (`self.Meshes`) (`self.Step 1`)) true :!label _label)
    (`KismetSystemLibrary.Delay` _stepduration)
    (if (not _damaged_2)
      (`SkinnedMeshComponent.SetSkinnedAssetAndUpdate` (`self.Mesh`) (`|GetArrayItem` (`self.Meshes`) (`self.Still`)) true)
      (`KismetSystemLibrary.Delay` _stepduration_2)
      (if (not _damaged)
        (`SkinnedMeshComponent.SetSkinnedAssetAndUpdate` (`self.Mesh`) (`|GetArrayItem` (`self.Meshes`) (`self.Step 2`)) true)
        (`KismetSystemLibrary.Delay` _stepduration_2)
        (if (not _damaged)
          (`SkinnedMeshComponent.SetSkinnedAssetAndUpdate` (`self.Mesh`) (`|GetArrayItem` (`self.Meshes`) (`self.Still`)) true :!label _label_2)
          (`KismetSystemLibrary.Delay` _stepduration)
          (if (not _damaged_2)
            (goto _label)))))))

(event `BeginWalk`
  (goto _label_2))

(event `self.ReceiveBeginPlay`
  (if (`self.Slide`)
    (`SkinnedMeshComponent.SetSkinnedAssetAndUpdate` (`self.Mesh`) (`|GetArrayItem` (`self.Meshes`) 5) true)
    (`KoopaMovementComponent.EnterSlide` (`self.KoopaMovementComponent`))
    (else
      (`self.BeginWalk`))))

(event `self.ReceiveTick`
  (params (DeltaSeconds :type "Float (single-precision)"))
  (if (not (`self.Slide`))
    (`self.AddMovementInput` (`SceneComponent.GetForwardVector` (`self.Mesh`)) 0.7)))

(fn `UserConstructionScript`)