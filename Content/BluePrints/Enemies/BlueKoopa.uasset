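; Blue Koopa enemy that walks or starts sliding, kicks shells and damages Mario on contact.
; Tick traces for cliffs and wall hits deflect its heading, while delay loops swap meshes as stepped animation.
; CatchBox catches kicked shells, absorbing momentum before dropping and kicking them back; the capsule handles idle shells or death by other shells.
; StompBox bounces Mario and destroys the Koopa, immediately on spin jumps or after a squash.
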(event `self.ReceiveBeginPlay`
  ;[0 0 0] Check if Koopa Should Slide or Walk on Begin Play
  (set `self.MovementVector` (`KismetMathLibrary.Normal` (`SceneComponent.GetForwardVector` (`self.Mesh`))))
  (if (`self.Slide`)
    (`SkinnedMeshComponent.SetSkinnedAssetAndUpdate` (`self.Mesh`) (`|GetArrayItem` (`self.Meshes`) 5) true)
    (else
      (`self.BeginWalk`))))

(event `BeginWalk`
  (bind _damaged (`self.Damaged`))
  (bind _stepduration (`self.StepDuration`))
  (bind _stepduration_2 (`self.StepDuration`))
  (bind _damaged_2 (`self.Damaged`))
  (set `CharacterMovementComponent.MaxWalkSpeed` 533.0 (`self.CharacterMovement`))
  (set `self.Damaged` false)
  (set `self.ShellPush` false)
  (`SkinnedMeshComponent.SetSkinnedAssetAndUpdate` (`self.Mesh`) (`|GetArrayItem` (`self.Meshes`) (`self.Still`)) true :!label _label)
  (`KismetSystemLibrary.Delay` _stepduration)
  (if (not _damaged_2)
    (`SkinnedMeshComponent.SetSkinnedAssetAndUpdate` (`self.Mesh`) (`|GetArrayItem` (`self.Meshes`) (`self.Step 1`)) true :!label _label_2)
    (`KismetSystemLibrary.Delay` _stepduration)
    (if (not _damaged_2)
      (`SkinnedMeshComponent.SetSkinnedAssetAndUpdate` (`self.Mesh`) (`|GetArrayItem` (`self.Meshes`) (`self.Still`)) true)
      (`KismetSystemLibrary.Delay` _stepduration_2)
      (if (not _damaged)
        (`SkinnedMeshComponent.SetSkinnedAssetAndUpdate` (`self.Mesh`) (`|GetArrayItem` (`self.Meshes`) (`self.Step 2`)) true)
        (`KismetSystemLibrary.Delay` _stepduration_2)
        (if (not _damaged)
          (goto _label))))))

(event `Stop Moving`
  (set `CharacterMovementComponent.MaxWalkSpeed` 0.0 (`self.CharacterMovement`))
  (set `self.Damaged` true)
  (`SkinnedMeshComponent.SetSkinnedAssetAndUpdate` (`self.Mesh`) (`|GetArrayItem` (`self.Meshes`) (`self.Still`)) false))

(event `EndSlide`
  (`SkinnedMeshComponent.SetSkinnedAssetAndUpdate` (`self.Mesh`) (`|GetArrayItem` (`self.Meshes`)) false)
  (`KismetSystemLibrary.Delay` 0.5)
  (set `self.Slide` false)
  (goto _label_2))

(event `self.ReceiveTick`
  (params (DeltaSeconds :type "Float (single-precision)"))
  (bind _returnvalue (`KismetMathLibrary.RandomFloatInRange` -0.5 0.5))
  (bind _mesh (`self.Mesh`))
  (bind _returnvalue_2 (`SceneComponent.K2_GetComponentRotation` _mesh))
  (bind _returnvalue_3 (`SceneComponent.K2_GetComponentLocation` _mesh))
  (if (`self.Slide`)
    (if (<= (`KismetMathLibrary.VSize` (`CharacterMovementComponent.GetLastUpdateVelocity` (`self.CharacterMovement`))) 10.0)
      (`self.EndSlide`))
    (elif (not (`self.ShellPush`))
      (bind (_outhit _returnvalue_4) (`KismetSystemLibrary.LineTraceSingleForObjects` _returnvalue_3 (+ _returnvalue_3 (* (+ (`KismetMathLibrary.GetForwardVector` _returnvalue_2) (* (`KismetMathLibrary.GetUpVector` _returnvalue_2) (0.0 0.0 -1.0))) (400.0 400.0 800.0))) (`self.CliffDetectionData`) true))
      (if _returnvalue_4
        (`self.AddMovementInput` (`self.MovementVector`) (`CharacterMovementComponent.MaxWalkSpeed` (`self.CharacterMovement`)))
        (else
          (bind _output_get (set `self.MovementVector` (+ (* (`self.MovementVector`) (-1.0 -1.0 0.0)) (`KismetMathLibrary.MakeVector` _returnvalue _returnvalue))))
          (`self.K2_SetActorRotation` (`KismetMathLibrary.Conv_VectorToRotator` _output_get)))))))

(event `self.CapsuleComponent.OnComponentBeginOverlap`
  (params (OverlappedComponent :type "PrimitiveComponent Object Reference") (OtherActor :type "Actor Object Reference") (OtherComp :type "PrimitiveComponent Object Reference") (OtherBodyIndex :type Integer) (bFromSweep :type Boolean) (SweepResult :type "HitResult Structure (by ref)"))
  (bind _shelltokick (`self.ShellToKick`))
  (bind _returnvalue (`KismetArrayLibrary.Array_Contains` (`PrimitiveComponent.GetOverlappingActors` (`self.CatchBox`) null) (`self.ShellToKick`)))
  (bind _asbp_mario (cast `/Game/BluePrints/BP_Mario` OtherActor)
    (:`then`
      (if (not (`self.Damaged`))
        (`/Engine/EditorBlueprintResources/StandardMacros.DoOnce` false
          (:`Completed`
            (`/Game/BluePrints/BP_Mario.TakeDamage` _asbp_mario false)))))
    (:`CastFailed`
      (bind _asshell (cast `/Game/BluePrints/Items/Shell` OtherActor))
      (switch `/Game/BluePrints/Enums/EHoldStates` (`/Game/BluePrints/Items/Shell.States` _asshell)
        (:`NewEnumerator0`
          (`self.Stop Moving`)
          (`KismetSystemLibrary.Delay` 0.5)
          (if _returnvalue
            (`/Game/BluePrints/Items/Shell.Calculate MoveVector` _shelltokick self)
            (`/Game/BluePrints/Items/Shell.Kick` _shelltokick self)
            (`SkinnedMeshComponent.SetSkinnedAssetAndUpdate` (`self.Mesh`) (`|GetArrayItem` (`self.Meshes`) 3) true)
            (`KismetSystemLibrary.Delay` 0.5)
            (`self.BeginWalk`)
            (else
              (`KismetSystemLibrary.Delay` 0.5)
              (`self.BeginWalk`))))
        (:`NewEnumerator1`
          (if (not _returnvalue)
            (`self.K2_DestroyActor` :!label _label_3)))
        (:`NewEnumerator3`
          (goto _label_3))
        (:`NewEnumerator2`
          (goto _label_3))
        (:`NewEnumerator4`
          (goto _label_3))))))

(event `self.CatchBox.OnComponentBeginOverlap`
  (params (OverlappedComponent :type "PrimitiveComponent Object Reference") (OtherActor :type "Actor Object Reference") (OtherComp :type "PrimitiveComponent Object Reference") (OtherBodyIndex :type Integer) (bFromSweep :type Boolean) (SweepResult :type "HitResult Structure (by ref)"))
  (bind (_returnvalue_x _returnvalue_y) (`KismetMathLibrary.BreakVector` (`self.K2_GetActorLocation`)))
  (bind _shelltokick (`self.ShellToKick`))
  (bind _shelltokick_2 (`self.ShellToKick`))
  (bind _shelltokick_3 (`self.ShellToKick`))
  (bind _charactermovement (`self.CharacterMovement`))
  (bind _shelltokick_4 (`self.ShellToKick`))
  (bind (_returnvalue_x_2 _returnvalue_y_2) (`KismetMathLibrary.BreakVector` (`self.K2_GetActorLocation` _shelltokick_3)))
  (bind (_returnvalue_x_3 _returnvalue_y_3) (`KismetMathLibrary.BreakVector` (`CharacterMovementComponent.GetLastUpdateVelocity` (`self.CharacterMovement`))))
  (bind _returnvalue (- (`KismetMathLibrary.MakeVector` _returnvalue_x_2 _returnvalue_y_2) (`KismetMathLibrary.MakeVector` _returnvalue_x _returnvalue_y)))
  (bind _asshell (cast `/Game/BluePrints/Items/Shell` OtherActor))
  (set `self.ShellToKick` _asshell)
  (switch `/Game/BluePrints/Enums/EHoldStates` (`/Game/BluePrints/Items/Shell.States` _asshell)
    (:`NewEnumerator1`
      (set `self.ShellPush` true)
      (`self.K2_SetActorRotation` self (`KismetMathLibrary.FindLookAtRotation` (`self.K2_GetActorLocation` self) (`self.K2_GetActorLocation` _asshell)) false)
      (`ActorComponent.SetActive` (`self.Spacer`) true true)
      (`SceneComponent.K2_AttachToComponent` (`Actor.RootComponent` _asshell) (`self.HoldBox`) "None" "SnapToTarget" "KeepRelative" "KeepWorld" false)
      (set `self.PushVector` (`/Game/BluePrints/Items/Shell.Impact Normal` _shelltokick))
      (set `/Game/BluePrints/Items/Shell.Impact Normal` (0.0 0.0 0.0) _shelltokick)
      (`self.Stop Moving`)
      (`/Engine/EditorBlueprintResources/StandardMacros.DoOnce` false :!label _label_4
        (:`Completed`
          (set `CharacterMovementComponent.BrakingDecelerationWalking` 2770.0 _charactermovement)
          (`CharacterMovementComponent.AddImpulse` _charactermovement (* (`self.PushVector`) (`self.MovementMultiplier`)) true)
          (`KismetSystemLibrary.Delay` 0.38)
          (`ActorComponent.SetActive` (`self.Spacer`) false true)
          (`SceneComponent.K2_DetachFromComponent` (`Actor.RootComponent` _shelltokick_3) "KeepWorld" "KeepWorld" "KeepWorld" true)
          (set `self.MovementVector` (`KismetMathLibrary.Normal` _returnvalue))
          (`CharacterMovementComponent.AddImpulse` (`self.CharacterMovement`) (* _returnvalue (3.33 3.33 1.0)) true)
          (set `/Game/BluePrints/Items/Shell.Moving` false _shelltokick_2)
          (set `/Game/BluePrints/Items/Shell.Launch Velocity` (`KismetMathLibrary.MakeVector` _returnvalue_x_3 _returnvalue_y_3) _shelltokick_2)
          (`KismetSystemLibrary.DelayUntilNextTick`)
          (`KismetSystemLibrary.DelayUntilNextTick`)
          (`KismetSystemLibrary.DelayUntilNextTick`)
          (`/Game/BluePrints/Items/Shell.Drop` _shelltokick_2 self)
          (`KismetSystemLibrary.Delay` 0.47)
          (`/Game/BluePrints/Items/Shell.Calculate MoveVector` _shelltokick_4 self)
          (`SkinnedMeshComponent.SetSkinnedAssetAndUpdate` (`self.Mesh`) (`|GetArrayItem` (`self.Meshes`) 3) true)
          (`KismetSystemLibrary.DelayUntilNextTick`)
          (`KismetSystemLibrary.DelayUntilNextTick`)
          (`/Game/BluePrints/Items/Shell.Kick` _shelltokick_4 self)
          (`KismetSystemLibrary.Delay` 0.4)
          (`self.BeginWalk`)
          (goto _label_4 :!via `Reset`))))))

(event `self.StompBox.OnComponentBeginOverlap`
  (params (OverlappedComponent :type "PrimitiveComponent Object Reference") (OtherActor :type "Actor Object Reference") (OtherComp :type "PrimitiveComponent Object Reference") (OtherBodyIndex :type Integer) (bFromSweep :type Boolean) (SweepResult :type "HitResult Structure (by ref)"))
  (bind _asbp_mario (cast `/Game/BluePrints/BP_Mario` OtherActor))
  (bind _output_get (set `self.As Mario` _asbp_mario))
  (`self.StopJumping` _output_get)
  (if (== (`/Game/BluePrints/BP_Mario.Shoebox` _asbp_mario) OtherComp)
    (set `self.Damaged` true)
    (if (`/Game/BluePrints/BP_Mario.SpinJumping` _output_get)
      (`/Engine/EditorBlueprintResources/StandardMacros.DoOnce` false
        (:`Completed`
          (`/Game/BluePrints/BP_Mario.EnemyBounce` (`self.As Mario`) false false 0)
          (`self.K2_DestroyActor`)))
      (else
        (`SkinnedMeshComponent.SetSkinnedAssetAndUpdate` (`self.Mesh`) (`|GetArrayItem` (`self.Meshes`) 6) true)
        (`CapsuleComponent.SetCapsuleSize` (`self.CapsuleComponent`) 35.0 35.0 true)
        (`/Engine/EditorBlueprintResources/StandardMacros.DoOnce` false
          (:`Completed`
            (`/Game/BluePrints/BP_Mario.EnemyBounce` (`self.As Mario`) false true 1)
            (set `CharacterMovementComponent.MaxWalkSpeed` 0.0 (`self.CharacterMovement`))
            (`KismetSystemLibrary.Delay` 0.5)
            (`self.K2_DestroyActor`)))))))

(event `self.CapsuleComponent.OnComponentHit`
  (params (HitComponent :type "PrimitiveComponent Object Reference") (OtherActor :type "Actor Object Reference") (OtherComp :type "PrimitiveComponent Object Reference") (NormalImpulse :type "Vector Structure") (Hit :type "HitResult Structure (by ref)"))
  (bind (_bblockinghit _binitialoverlap _time _distance _location _impactpoint _normal _impactnormal) (`GameplayStatics.BreakHitResult` Hit))
  (bind _returnvalue (`KismetMathLibrary.RandomFloatInRange` -0.5 0.5))
  (bind _returnvalue_2 (`self.K2_GetActorLocation`))
  ;[1 1 1] TurnAround
  (if (and (not (`self.Slide`)) (>= (`KismetMathLibrary.Round` (`KismetMathLibrary.DegAcos` (`KismetMathLibrary.Dot_VectorVector` _impactnormal (0.0 0.0 1.0)))) 90))
    (`/Engine/EditorBlueprintResources/StandardMacros.DoOnce` false :!label _label_5
      (:`Completed`
        (bind _output_get (set `self.MovementVector` (`KismetMathLibrary.Normal` (+ (`KismetMathLibrary.MirrorVectorByNormal` (`self.MovementVector`) (`KismetMathLibrary.MakeVector` (.x _normal) (.y _normal))) (`KismetMathLibrary.MakeVector` _returnvalue _returnvalue)))))
        (`self.K2_SetActorRotation` (`KismetMathLibrary.FindLookAtRotation` _returnvalue_2 (+ _returnvalue_2 _output_get)))
        (`KismetSystemLibrary.Delay` 0.2)
        (goto _label_5 :!via `Reset`)))))

(fn `UserConstructionScript`)