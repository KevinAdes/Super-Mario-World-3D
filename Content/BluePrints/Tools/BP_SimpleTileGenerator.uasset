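; BP_SimpleTileGenerator is a tool Blueprint that tiles a chosen static mesh into a hollow box.
; The construction script loops over an Xnum by Ynum by Znum grid and adds a BlockToTile mesh component only on the outer faces, at a fixed spacing.
; An IsBetween range helper with optional inclusive bounds is defined but not called, and the event graph is empty.
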(fn `isBetween`
  (params (Max :type Integer) (Min :type Integer) (Num :type Integer) (`Max Inclusive` :type Boolean) (`Min Inclusive` :type Boolean))
  (returns (True :type Boolean))
  (return (and (select `bool` `Min Inclusive` :`false` (> Num Min) :`true` (>= Num Min)) (select `bool` `Max Inclusive` :`false` (< Num Max) :`true` (<= Num Max)))))

(fn `UserConstructionScript`
  (locals (TempSMC :type "StaticMeshComponent Object Reference"))
  (bind _returnvalue (- (`self.Znum`) 1))
  (bind _returnvalue_2 (- (`self.Xnum`) 1))
  (bind _returnvalue_3 (- (`self.Ynum`) 1))
  (for _index (range (+ _returnvalue_2 1))
    (for _index_2 (range (+ _returnvalue_3 1))
      (for _index_3 (range (+ _returnvalue 1))
        (if (or (or (== _index 0) (== _index _returnvalue_2)) (or (== _index_2 0) (== _index_2 _returnvalue_3)) (or (== _index_3 0) (== _index_3 _returnvalue)))
          (bind _returnvalue_4 (`AddComponent|NODE_AddStaticMeshComponent-0` :`self` self :`RelativeTransform` (`KismetMathLibrary.MakeTransform` (* (`KismetMathLibrary.MakeVector` (`KismetMathLibrary.Conv_IntToDouble` _index) (`KismetMathLibrary.Conv_IntToDouble` _index_2) (`KismetMathLibrary.Conv_IntToDouble` _index_3)) 160))))
          (`StaticMeshComponent.SetStaticMesh` _returnvalue_4 (`self.BlockToTile`)))))))