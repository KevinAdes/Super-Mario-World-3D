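; Player state for a Mario game that tracks lives, coins, points and star points, and handles switching between the map and levels.
; LoadLevel and LoadMap stream level instances and request the other's unload, with a loading screen for levels.
; Load callbacks swap the possessed pawn between BP_MapMario (spawned behind a DoOnce) and BP_Mario, whose spawn pauses the game.
; Counter gains fire dispatchers, and 100 coins grant a life.
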(event `self.ReceiveBeginPlay`
  (bind _returnvalue (`|CreateWidget` "/Game/BluePrints/Widgets/HUD/WBP_LoadingScreen.WBP_LoadingScreen_C"))
  (set `self.LoadingScreen` _returnvalue)
  (`UserWidget.AddToViewport` _returnvalue 0))

(fn `AddLife`
  (bind _result (`/Engine/EditorBlueprintResources/StandardMacros.IncrementInt` (`self.Lives`))
    (:`  `
      (`self.OnLifeAdded` _result))))

(fn `AddPoints`
  (params (NumToAdd :type Integer))
  (bind _output_get (set `self.Points` (+ (stale _output_get) NumToAdd)))
  (`self.OnPointsAdded` _output_get))

(fn `AddStarPoints`
  (`/Engine/EditorBlueprintResources/StandardMacros.IncrementInt` (`self.BP_StarPoints`)
    (:`  `
      (`self.OnStarPointsAdded`))))

(fn `CollectCoin`
  (`|ExecutionSequence`
    (:`then_0`
      (`/Engine/EditorBlueprintResources/StandardMacros.IncrementInt` (`self.Coins`)))
    (:`then_1`
      (if (== (`self.Coins`) 100)
        (`self.AddLife`)
        (set `self.Coins` 0)))
    (:`then_2`
      (`self.OnCoinCollected` (`self.Coins`)))))

(fn `LoadLevel`
  (params (LevelName :type String))
  (bind _loadingscreen (`self.LoadingScreen`))
  (`|ExecutionSequence`
    (:`then_0`
      (`/Game/BluePrints/Widgets/HUD/WBP_LoadingScreen.SetVisible` _loadingscreen true)
      (`/Game/BluePrints/Widgets/HUD/WBP_LoadingScreen.LoadGameStartScreen` _loadingscreen))
    (:`then_1`
      (bind _maplevelreference (`self.MapLevelReference`)
        (:`then`
          (`LevelStreaming.SetIsRequestingUnloadAndRemoval` _maplevelreference true))
        (:`else`)))
    (:`then_2`
      (set `self.Level Name` LevelName)
      (set `self.CurrentLevelName` (`KismetStringLibrary.Conv_StringToName` LevelName))
      (bind (_boutsuccess _returnvalue) (`LevelStreamingDynamic.LoadLevelInstance` LevelName (0.0 0.0 0.0) (struct) "" null))
      (set `self.LevelReference` _returnvalue)
      (add `LevelStreaming.OnLevelLoaded` _returnvalue (`|CreateDelegate` :!event `OnLevelLoaded`)))))

(fn `LoadMap`
  (params (LevelName :type String))
  (`|ExecutionSequence`
    (:`then_0`
      (bind _outactors (`GameplayStatics.GetAllActorsOfClass` "/Game/BluePrints/GameStuff/BP_SMWCamera.BP_SMWCamera_C"))
      (for _array_element _outactors
        (`self.K2_DestroyActor` _array_element)))
    (:`then_1`
      (bind _levelreference (`self.LevelReference`)
        (:`then`
          (`LevelStreaming.SetIsRequestingUnloadAndRemoval` _levelreference true))
        (:`else`)))
    (:`then_2`
      (bind (_boutsuccess _returnvalue) (`LevelStreamingDynamic.LoadLevelInstance` (`self.Map Name`) (0.0 0.0 0.0) (struct) "" null))
      (set `self.MapLevelReference` _returnvalue)
      (add `LevelStreaming.OnLevelLoaded` _returnvalue (`|CreateDelegate` :!event `OnMapLoaded`)))))

(fn `OnLevelLoaded`
  (`|ExecutionSequence`
    (:`then_0`
      (bind _outactors (`GameplayStatics.GetAllActorsOfClass` "/Game/BluePrints/Map/BP_MapMario.BP_MapMario_C"))
      (for _array_element _outactors
        (`/Game/BluePrints/Map/BP_MapMario.Destruct` _array_element)))
    (:`then_2`
      (`GameplayStatics.SetGamePaused` true)
      (bind _returnvalue (`|SpawnActorFromClass` "/Game/BluePrints/BP_Mario.BP_Mario_C" (`KismetMathLibrary.MakeTransform` (0.0 0.0 1000.0)) "Undefined" "MultiplyWithRoot" null true null))
      (`Controller.Possess` (`GameplayStatics.GetPlayerController` 0) _returnvalue))))

(fn `OnMapLoaded`
  (`|ExecutionSequence`
    (:`then_0`
      (bind _outactors (`GameplayStatics.GetAllActorsOfClass` "/Game/BluePrints/BP_Mario.BP_Mario_C"))
      (for _array_element _outactors
        (`/Game/BluePrints/BP_Mario.Destruct` _array_element)))
    (:`then_1`
      (`/Engine/EditorBlueprintResources/StandardMacros.DoOnce` false
        (:`Completed`
          (bind _returnvalue (`|SpawnActorFromClass` "/Game/BluePrints/Map/BP_MapMario.BP_MapMario_C" (`KismetMathLibrary.MakeTransform` (0.0 0.0 0.0)) "Undefined" "MultiplyWithRoot" null null))
          (`Controller.Possess` (`GameplayStatics.GetPlayerController` 0) _returnvalue))))))

(fn `RemoveLife`
  (`/Engine/EditorBlueprintResources/StandardMacros.DecrementInt` (`self.Lives`)))

(fn `UnloadLevel`)

(fn `UnloadMap`)

(fn `UserConstructionScript`)